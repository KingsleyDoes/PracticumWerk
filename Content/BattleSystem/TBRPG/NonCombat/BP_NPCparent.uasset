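; BP_NPCparent is the base non-combat NPC for the TBRPG free-roam mode, showing dialogue when interacted with.
; Interact creates a W_NPCspeech widget from the NPC's name and dialogue lines and adds it to the viewport.
; The widget is removed when BP_FreeRoamGalypso stops overlapping the Box.
; BeginPlay caches a Galypso reference, and GetCompleted always returns false.
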(event `self.ReceiveBeginPlay`
  (bind _returnvalue (`GameplayStatics.GetActorOfClass` "/Game/BattleSystem/TBRPG/NonCombat/BP_FreeRoamGalypso.BP_FreeRoamGalypso_C"))
  (set `self.Gal` _returnvalue))

(event `/Game/demopixelassets/blueprintsfordemo/InterfacesAndComponenets/BPI_Interact.Interact`
  (params (Player :type "Actor Object Reference"))
  (`/Engine/EditorBlueprintResources/StandardMacros.IsValid` Player
    (:`Is Valid`
      (bind _returnvalue (`|CreateWidget` "/Game/BattleSystem/TBRPG/UI/W_NPCspeech.W_NPCspeech_C" (`GameplayStatics.GetPlayerController` 0) (`self.NPCdialogueLines`) (`self.NPCName`)))
      (bind _output_get (set `self.NPCwidget` _returnvalue))
      (`UserWidget.AddToViewport` _output_get 0))))

(event `self.Box.OnComponentEndOverlap`
  (params (OverlappedComponent :type "PrimitiveComponent Object Reference") (OtherActor :type "Actor Object Reference") (OtherComp :type "PrimitiveComponent Object Reference") (OtherBodyIndex :type Integer))
  (cast `/Game/BattleSystem/TBRPG/NonCombat/BP_FreeRoamGalypso` OtherActor)
  (`Widget.RemoveFromParent` (`self.NPCwidget`)))

(fn `GetCompleted`
  (returns (Completed :type Boolean))
  (return false))

(fn `UserConstructionScript`)