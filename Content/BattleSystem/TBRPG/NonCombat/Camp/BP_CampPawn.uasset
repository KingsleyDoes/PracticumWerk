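; BP_CampPawn is the camp pawn for the TBRPG non-combat camp, handling what happens when the party rests.
; RestTriggered adjusts a PercentChance value based on the WatchSlot, then runs Goodnight.
; Goodnight passes the two tent slot occupants to BoostRelationship, whose body is still empty, so resting has no relationship effect yet.
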(event `RestTriggered`
  (if (== (`self.WatchSlot`) null)
    (set `self.PercentChance` (+ 0.5 (`self.PercentChance`))))
  (`self.Goodnight`))

(event `Goodnight`
  (`self.BoostRelationship` (`self.TentSlot1`) (`self.TentSlot2`)))

(event `BoostRelationship`
  (params (Character1 :type "/Game/BattleSystem/TBRPG/Combat/CharactersBlueprints/BP_PawnBase Object Reference") (Character2 :type "/Game/BattleSystem/TBRPG/Combat/CharactersBlueprints/BP_PawnBase Object Reference")))

(fn `UserConstructionScript`)