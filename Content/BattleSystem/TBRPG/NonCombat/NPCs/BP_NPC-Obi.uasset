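; NPC Obi for a scripted free-roam scene that runs a trio in and leads into the move to the village.
; On BeginPlay it freezes the player, BP_FreeRoamGalypso, while a timeline slides the actor in and switches Obi, Mehzia and Niren from run to idle flipbooks.
; Interact opens a one-time W_NPCspeech dialogue.
; When its lines finish, FadeToVillage fades the camera out, teleports the player, fades back in and unfreezes them.
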(event `self.ReceiveBeginPlay`
  (`parent.ReceiveBeginPlay`)
  (`|ExecutionSequence`
    (:`then_0`
      (`PaperFlipbookComponent.SetFlipbook` (`self.Sprite`) "/Game/BattleSystem/TBRPG/PixelAssets/CharacterArt/obi/obi-sprite-run.obi-sprite-run")
      (`PaperFlipbookComponent.SetFlipbook` (`self.Mehzia`) "/Game/BattleSystem/TBRPG/PixelAssets/CharacterArt/Mehzia/mehzia-sprite-run.mehzia-sprite-run")
      (`PaperFlipbookComponent.SetFlipbook` (`self.Niren`) "/Game/BattleSystem/TBRPG/PixelAssets/CharacterArt/niren/niren-testsprite-run1.niren-testsprite-run1")
      (bind (_direction _newtrack_0) (`Timeline|Run In` :!via `PlayFromStart`)
        (:`Update`
          (`self.K2_SetActorLocation` (`KismetMathLibrary.VLerp` (13800.0 10.0 -3242.0) (9290.0 10.0 -3242.0) _newtrack_0)))
        (:`Finished`
          (`PaperFlipbookComponent.SetFlipbook` (`self.Sprite`) "/Game/BattleSystem/TBRPG/PixelAssets/CharacterArt/obi/obi-sprite-idle.obi-sprite-idle")
          (`PaperFlipbookComponent.SetFlipbook` (`self.Mehzia`) "/Game/BattleSystem/TBRPG/PixelAssets/CharacterArt/Mehzia/mehzia-sprite-idle.mehzia-sprite-idle")
          (`PaperFlipbookComponent.SetFlipbook` (`self.Niren`) "/Game/BattleSystem/TBRPG/PixelAssets/CharacterArt/niren/niren-testsprite-idle1.niren-testsprite-idle1"))))
    (:`then_1`
      (bind _returnvalue (`GameplayStatics.GetActorOfClass` "/Game/BattleSystem/TBRPG/NonCombat/BP_FreeRoamGalypso.BP_FreeRoamGalypso_C"))
      (set `/Game/BattleSystem/TBRPG/NonCombat/BP_FreeRoamGalypso.Frozen` true _returnvalue))))

(event `/Game/demopixelassets/blueprintsfordemo/InterfacesAndComponenets/BPI_Interact.Interact`
  (params (Player :type "Actor Object Reference"))
  (`/Engine/EditorBlueprintResources/StandardMacros.IsValid` Player
    (:`Is Valid`
      (`/Engine/EditorBlueprintResources/StandardMacros.DoOnce` false
        (:`Completed`
          (bind _returnvalue (`|CreateWidget` "/Game/BattleSystem/TBRPG/UI/W_NPCspeech.W_NPCspeech_C" (`GameplayStatics.GetPlayerController` 0) (`self.NPCdialogueLines`) (`self.NPCName`) "/Game/BattleSystem/TBRPG/NonCombat/Camp/pxlportraits-obi.pxlportraits-obi"))
          (bind _output_get (set `self.NPCwidget` _returnvalue))
          (`UserWidget.AddToViewport` _output_get 0)
          (add `/Game/BattleSystem/TBRPG/UI/W_NPCspeech.LinesFinished` _output_get (delegate `FadeToVillage`)))))))

(event `FadeToVillage`
  (bind _returnvalue (`GameplayStatics.GetPlayerCameraManager` 0))
  (`PlayerCameraManager.StartCameraFade` _returnvalue 0.0 1.0 1.0 (struct :`R` 0.020289 :`G` 0.006995 :`B` 0.012286 :`A` 1.0) false true)
  (`KismetSystemLibrary.Delay` 1.0)
  (bind _returnvalue_2 (`GameplayStatics.GetActorOfClass` "/Game/BattleSystem/TBRPG/NonCombat/BP_FreeRoamGalypso.BP_FreeRoamGalypso_C"))
  (`self.K2_SetActorLocation` _returnvalue_2 (19220.0 10.0 -2370.0) false false)
  (`KismetSystemLibrary.Delay` 1.0)
  (`PlayerCameraManager.StartCameraFade` _returnvalue 1.0 0.0 1.0 (struct :`R` 0.020289 :`G` 0.006995 :`B` 0.012286 :`A` 1.0) false true)
  (`KismetSystemLibrary.Delay` 1.0)
  (`PlayerCameraManager.StopCameraFade` _returnvalue)
  (set `/Game/BattleSystem/TBRPG/NonCombat/BP_FreeRoamGalypso.Frozen` false _returnvalue_2))

(fn `UserConstructionScript`
  (`parent.UserConstructionScript`))