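; Villager NPC Blueprint for Uzomma, a female townsperson in the non-combat side of the turn-based RPG, extending a parent NPC class.
; BeginPlay runs the parent logic, then sets her sprite flipbook and name.
; Interact checks the player is valid, then creates and displays a speech widget with her dialogue lines, name and portrait.
; A DoOnce gates the widget, and this graph never resets it.
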(event `self.ReceiveBeginPlay`
  (`parent.ReceiveBeginPlay`)
  (`PaperFlipbookComponent.SetFlipbook` (`self.Sprite`) "/Game/BattleSystem/TBRPG/PixelAssets/CharacterArt/NPC/FB_NPC_F3.FB_NPC_F3")
  (set `self.NPCName` "Uzomma") ; female
)

(event `self.Interact`
  (params (Player :type "Actor Object Reference"))
  (`/Engine/EditorBlueprintResources/StandardMacros.IsValid` Player
    (:`Is Valid`
      (`/Engine/EditorBlueprintResources/StandardMacros.DoOnce` false
        (:`Completed`
          (bind _returnvalue (`|CreateWidget` "/Game/BattleSystem/TBRPG/UI/W_NPCspeech.W_NPCspeech_C" (`GameplayStatics.GetPlayerController` 0) (`self.NPCdialogueLines`) (`self.NPCName`) "/Game/BattleSystem/TBRPG/PixelAssets/CharacterArt/NPC/pxlportraits-NPCuzomma.pxlportraits-NPCuzomma"))
          (bind _output_get (set `self.NPCwidget` _returnvalue))
          (`UserWidget.AddToViewport` _output_get 0))))))

(fn `UserConstructionScript`
  (`parent.UserConstructionScript`))