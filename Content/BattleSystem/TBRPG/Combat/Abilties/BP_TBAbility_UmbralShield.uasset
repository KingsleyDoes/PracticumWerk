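; Umbral Shield ability for the turn-based RPG, in which an enemy pawn applies a one-turn DEF effect to itself.
; It casts the executing actor to the Hittake enemy parent and calls its UmbralShield before committing the ability.
; On commit, timed delays sequence the self-effect, a status update with CheckStatus, and EndAbility.
; A failed cast or commit never reaches EndAbility.
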(event `self.ActivateAbility`
  (params (ExecutingActor :type "/Game/BattleSystem/TBRPG/Combat/CharactersBlueprints/BP_PawnBase Object Reference"))
  (bind _asbp_pawn_base_enemy_parent_hittake (cast `/Game/BattleSystem/TBRPG/Combat/CharactersBlueprints/Enemies/BP_PawnBase_EnemyParent_Hittake` ExecutingActor))
  (`/Game/BattleSystem/TBRPG/Combat/CharactersBlueprints/Enemies/BP_PawnBase_EnemyParent_Hittake.UmbralShield` _asbp_pawn_base_enemy_parent_hittake)
  (bind _comitted (`self.CommitAbility`))
  (if _comitted
    (`KismetSystemLibrary.Delay` 0.2)
    (`/Game/BattleSystem/TBRPG/Combat/Abilties/AC_AbilityComponent.AffectSelf` (`self.OwningAbilityComponent`) "NewEnumerator1" "DEF" "NewEnumerator5" "NewEnumerator0" 35.0 1)
    (set `/Game/BattleSystem/TBRPG/Combat/Abilties/AC_AbilityComponent.CurrentStatus` "NewEnumerator5" (`self.OwningAbilityComponent`))
    (`/Game/BattleSystem/TBRPG/Combat/CharactersBlueprints/BP_PawnBase.CheckStatus` _asbp_pawn_base_enemy_parent_hittake)
    (`KismetSystemLibrary.Delay` 0.5)
    (`self.EndAbility`)))

(fn `UserConstructionScript`
  (`parent.UserConstructionScript`))