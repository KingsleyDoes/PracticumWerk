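; Turn-based combat ability that makes a Sporemonger enemy burst and damage its target's LP.
; On activation it casts the executor to the Sporemonger, triggers its Burst, then commits the ability.
; It sends a hit reaction to the target, rolls random damage filtered through the target's defense, shows the number and applies it to LP before ending.
; Short delays pace the hit, damage and end steps.
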(event `self.ActivateAbility`
  (params (ExecutingActor :type "/Game/BattleSystem/TBRPG/Combat/CharactersBlueprints/BP_PawnBase Object Reference"))
  (bind _owningabilitycomponent (`self.OwningAbilityComponent`))
  (bind _targactor (`/Game/BattleSystem/TBRPG/Combat/Abilties/AC_AbilityComponent.TargActor` _owningabilitycomponent))
  (bind _asbp_pawn_base_enemy_parent_sporemonger (cast `/Game/BattleSystem/TBRPG/Combat/CharactersBlueprints/Enemies/BP_PawnBase_EnemyParent_Sporemonger` ExecutingActor))
  (`/Game/BattleSystem/TBRPG/Combat/CharactersBlueprints/Enemies/BP_PawnBase_EnemyParent_Sporemonger.Burst` _asbp_pawn_base_enemy_parent_sporemonger)
  (bind _comitted (`self.CommitAbility`))
  (if _comitted
    (bind _component (message `/Game/BattleSystem/TBRPG/Combat/BPI_TurnBasedCombat.GetAbilityComponent` _targactor))
    (bind _output_get (set `self.AbilityEnum` "NewEnumerator1"))
    (`/Game/BattleSystem/TBRPG/Combat/CharactersBlueprints/BP_PawnBase.GetHit` _targactor _output_get)
    (`KismetSystemLibrary.Delay` 0.3)
    (bind _outputdamage (`self.ApplyDefense` _component (`KismetMathLibrary.RandomIntegerInRange` -15 -5)))
    (`/Game/BattleSystem/TBRPG/Combat/CharactersBlueprints/BP_PawnBase.ShowDamage` _targactor (`KismetMathLibrary.FTrunc` _outputdamage))
    (`/Game/BattleSystem/TBRPG/Combat/Abilties/AC_AbilityComponent.ApplyEffectToTarget` _owningabilitycomponent "NewEnumerator0" _component "LP" "NewEnumerator4" "NewEnumerator0" _outputdamage 0)
    (`KismetSystemLibrary.Delay` 0.1)
    (`self.EndAbility`)))

(fn `UserConstructionScript`
  (`parent.UserConstructionScript`))