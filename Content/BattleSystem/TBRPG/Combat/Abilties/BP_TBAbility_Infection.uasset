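; Turn-based RPG ability for the Sporemonger enemy that infects its target.
; It calls the Sporemonger's Infection event, commits, then triggers GetHit on the target and, shortly after, on the Sporemonger.
; It applies a random negative magnitude, adjusted by ApplyDefense, to the target.
; A second two-turn effect with a separately rolled positive magnitude is applied without an explicit target component, then the ability ends.
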(event `self.ActivateAbility`
  (params (ExecutingActor :type "/Game/BattleSystem/TBRPG/Combat/CharactersBlueprints/BP_PawnBase Object Reference"))
  (bind _returnvalue (`KismetMathLibrary.RandomIntegerInRange` -10 -5))
  (bind _owningabilitycomponent (`self.OwningAbilityComponent`))
  (bind _targactor (`/Game/BattleSystem/TBRPG/Combat/Abilties/AC_AbilityComponent.TargActor` _owningabilitycomponent))
  (bind _asbp_pawn_base_enemy_parent_sporemonger (cast `/Game/BattleSystem/TBRPG/Combat/CharactersBlueprints/Enemies/BP_PawnBase_EnemyParent_Sporemonger` ExecutingActor))
  (`/Game/BattleSystem/TBRPG/Combat/CharactersBlueprints/Enemies/BP_PawnBase_EnemyParent_Sporemonger.Infection` _asbp_pawn_base_enemy_parent_sporemonger)
  (bind _comitted (`self.CommitAbility`))
  (if _comitted
    (bind _component (message `/Game/BattleSystem/TBRPG/Combat/BPI_TurnBasedCombat.GetAbilityComponent` _targactor))
    (bind _output_get (set `self.AbilityEnum` "NewEnumerator12"))
    (`/Game/BattleSystem/TBRPG/Combat/CharactersBlueprints/BP_PawnBase.GetHit` _targactor _output_get)
    (`KismetSystemLibrary.Delay` 0.3)
    (bind _output_get_2 (set `self.AbilityEnum` "NewEnumerator12"))
    (`/Game/BattleSystem/TBRPG/Combat/CharactersBlueprints/BP_PawnBase.GetHit` _asbp_pawn_base_enemy_parent_sporemonger _output_get_2)
    (bind _outputdamage (`self.ApplyDefense` _component _returnvalue))
    (`/Game/BattleSystem/TBRPG/Combat/Abilties/AC_AbilityComponent.ApplyEffectToTarget` _owningabilitycomponent "NewEnumerator0" _component "DEF" "NewEnumerator4" "NewEnumerator0" _outputdamage 0)
    (`/Game/BattleSystem/TBRPG/Combat/Abilties/AC_AbilityComponent.ApplyEffectToTarget` _owningabilitycomponent "NewEnumerator1" null "DEF" "NewEnumerator5" "NewEnumerator0" (`KismetMathLibrary.Conv_IntToDouble` (* _returnvalue -2)) 2)
    (`KismetSystemLibrary.Delay` 0.1)
    (`self.EndAbility`)))

(fn `UserConstructionScript`
  (`parent.UserConstructionScript`))