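; Turn-based combat ability that lets the Morchella enemy recompose, affecting its own DEF and LP.
; On activation it casts the executing actor to Morchella and calls its Recompose before committing the ability.
; After a successful commit and short delay, it applies a one-turn DEF effect and an LP effect through the owning ability component.
; It then sets the component's status, has the pawn check it, and ends after another delay.
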(event `self.ActivateAbility`
  (params (ExecutingActor :type "/Game/BattleSystem/TBRPG/Combat/CharactersBlueprints/BP_PawnBase Object Reference"))
  (bind _owningabilitycomponent (`self.OwningAbilityComponent`))
  (bind _asbp_pawn_base_enemy_parent_morchella (cast `/Game/BattleSystem/TBRPG/Combat/CharactersBlueprints/Enemies/BP_PawnBase_EnemyParent_Morchella` ExecutingActor))
  (`/Game/BattleSystem/TBRPG/Combat/CharactersBlueprints/Enemies/BP_PawnBase_EnemyParent_Morchella.Recompose` _asbp_pawn_base_enemy_parent_morchella)
  (bind _comitted (`self.CommitAbility`))
  (if _comitted
    (`KismetSystemLibrary.Delay` 0.2)
    (`/Game/BattleSystem/TBRPG/Combat/Abilties/AC_AbilityComponent.AffectSelf` _owningabilitycomponent "NewEnumerator1" "DEF" "NewEnumerator5" "NewEnumerator0" 25.0 1)
    (`/Game/BattleSystem/TBRPG/Combat/Abilties/AC_AbilityComponent.AffectSelf` _owningabilitycomponent "NewEnumerator0" "LP" "NewEnumerator4" "NewEnumerator0" 25.0 0)
    (set `/Game/BattleSystem/TBRPG/Combat/Abilties/AC_AbilityComponent.CurrentStatus` "NewEnumerator5" (`self.OwningAbilityComponent`))
    (`/Game/BattleSystem/TBRPG/Combat/CharactersBlueprints/BP_PawnBase.CheckStatus` _asbp_pawn_base_enemy_parent_morchella)
    (`KismetSystemLibrary.Delay` 0.5)
    (`self.EndAbility`)))

(fn `UserConstructionScript`
  (`parent.UserConstructionScript`))