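; Turn-based RPG enemy ability Spike Rain, usable only by a Cractus enemy pawn.
; On activation it calls the Cractus's SpikeRain, then attempts to commit the ability.
; If committed, it triggers GetHit on the ability component's target actor, applies a fixed LP reduction after a short delay, then ends the ability after another delay.
; A failed cast or commit stops the flow without calling EndAbility.
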(event `self.ActivateAbility`
  (params (ExecutingActor :type "/Game/BattleSystem/TBRPG/Combat/CharactersBlueprints/BP_PawnBase Object Reference"))
  (bind _owningabilitycomponent (`self.OwningAbilityComponent`))
  (bind _targactor (`/Game/BattleSystem/TBRPG/Combat/Abilties/AC_AbilityComponent.TargActor` _owningabilitycomponent))
  (bind _asbp_pawn_base_enemy_parent_cractus (cast `/Game/BattleSystem/TBRPG/Combat/CharactersBlueprints/Enemies/BP_PawnBase_EnemyParent_Cractus` ExecutingActor))
  (`/Game/BattleSystem/TBRPG/Combat/CharactersBlueprints/Enemies/BP_PawnBase_EnemyParent_Cractus.SpikeRain` _asbp_pawn_base_enemy_parent_cractus)
  (bind _comitted (`self.CommitAbility`))
  (if _comitted
    (bind _component (message `/Game/BattleSystem/TBRPG/Combat/BPI_TurnBasedCombat.GetAbilityComponent` _targactor))
    (`/Game/BattleSystem/TBRPG/Combat/CharactersBlueprints/BP_PawnBase.GetHit` _targactor "Spike Rain")
    (`KismetSystemLibrary.Delay` 0.2)
    (`/Game/BattleSystem/TBRPG/Combat/Abilties/AC_AbilityComponent.ApplyEffectToTarget` _owningabilitycomponent "NewEnumerator0" _component "LP" "NewEnumerator4" "NewEnumerator0" -15.0 0)
    (`KismetSystemLibrary.Delay` 0.5)
    (`self.EndAbility`)))

(fn `UserConstructionScript`
  (`parent.UserConstructionScript`))