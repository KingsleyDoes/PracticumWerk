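; BP_TBAbility_Uplift is a turn-based RPG combat ability that applies a fixed BP attribute effect to the targeted actor.
; Once committed, it plays an effect flipbook on the target, spawns a Niagara system at its location and applies the effect through both actors' ability components.
; After a short delay it clears the flipbook and ends the ability.
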(event `self.ActivateAbility`
  (bind _owningabilitycomponent (`self.OwningAbilityComponent`))
  (bind _targactor (`/Game/BattleSystem/TBRPG/Combat/Abilties/AC_AbilityComponent.TargActor` _owningabilitycomponent))
  (bind _effectanimation (`/Game/BattleSystem/TBRPG/Combat/CharactersBlueprints/BP_PawnBase.EffectAnimation` _targactor))
  (bind _comitted (`self.CommitAbility`))
  (if _comitted
    (`PaperFlipbookComponent.SetFlipbook` _effectanimation (`self.EffectFlipbook`))
    (bind _component (message `/Game/BattleSystem/TBRPG/Combat/BPI_TurnBasedCombat.GetAbilityComponent` _targactor))
    (`NiagaraFunctionLibrary.SpawnSystemAtLocation` (`self.NiagaraSys`) (`self.K2_GetActorLocation` _targactor))
    (`/Game/BattleSystem/TBRPG/Combat/Abilties/AC_AbilityComponent.ApplyEffectToTarget` _owningabilitycomponent "NewEnumerator0" _component "BP" "NewEnumerator4" "NewEnumerator0" 10.0 0)
    (`KismetSystemLibrary.Delay` 2.0)
    (`PaperFlipbookComponent.SetFlipbook` _effectanimation null)
    (`self.EndAbility`)))

(fn `UserConstructionScript`
  (`parent.UserConstructionScript`))