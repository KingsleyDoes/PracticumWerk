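; Turn-based combat ability for the Mega Spore Blast attack, used by pawns derived from the enemy hit-take parent.
; Activation calls the caster's MegaSporeBlast before committing, then sends the target a hit reaction.
; After a short delay, it passes a random negative damage roll through defense, applies it to the target's LP and shows the number.
; The ability ends after a second delay.
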(event `self.ActivateAbility`
  (params (ExecutingActor :type "/Game/BattleSystem/TBRPG/Combat/CharactersBlueprints/BP_PawnBase Object Reference"))
  (bind _owningabilitycomponent (`self.OwningAbilityComponent`))
  (bind _targactor (`/Game/BattleSystem/TBRPG/Combat/Abilties/AC_AbilityComponent.TargActor` _owningabilitycomponent))
  (bind _asbp_pawn_base_enemy_parent_hittake (cast `/Game/BattleSystem/TBRPG/Combat/CharactersBlueprints/Enemies/BP_PawnBase_EnemyParent_Hittake` ExecutingActor))
  (`/Game/BattleSystem/TBRPG/Combat/CharactersBlueprints/Enemies/BP_PawnBase_EnemyParent_Hittake.MegaSporeBlast` _asbp_pawn_base_enemy_parent_hittake)
  (bind _comitted (`self.CommitAbility`))
  (if _comitted
    (bind _component (message `/Game/BattleSystem/TBRPG/Combat/BPI_TurnBasedCombat.GetAbilityComponent` _targactor))
    (bind _output_get (set `self.AbilityEnum` "NewEnumerator12"))
    (`/Game/BattleSystem/TBRPG/Combat/CharactersBlueprints/BP_PawnBase.GetHit` _targactor _output_get)
    (`KismetSystemLibrary.Delay` 0.2)
    (bind _outputdamage (`self.ApplyDefense` _component (`KismetMathLibrary.RandomIntegerInRange` -25 -20)))
    (`/Game/BattleSystem/TBRPG/Combat/Abilties/AC_AbilityComponent.ApplyEffectToTarget` _owningabilitycomponent "NewEnumerator0" _component "LP" "NewEnumerator4" "NewEnumerator0" _outputdamage 0)
    (`/Game/BattleSystem/TBRPG/Combat/CharactersBlueprints/BP_PawnBase.ShowDamage` _targactor (`KismetMathLibrary.FTrunc` _outputdamage))
    (`KismetSystemLibrary.Delay` 0.5)
    (`self.EndAbility`)))

(fn `UserConstructionScript`
  (`parent.UserConstructionScript`))