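; Illuminate is a turn-based combat ability for the Galypso player pawn that hits the current target and applies a timed BP effect.
; On activation it casts the executor to Galypso, plays the Illuminate animation, then commits.
; If committed, it triggers the target's hit reaction and applies a small random LP loss filtered through defense.
; A second effect modifies BP by a 0.5 magnitude for two turns before the ability ends.
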(event `self.ActivateAbility`
  (params (ExecutingActor :type "/Game/BattleSystem/TBRPG/Combat/CharactersBlueprints/BP_PawnBase Object Reference"))
  (bind _owningabilitycomponent (`self.OwningAbilityComponent`))
  (bind _targactor (`/Game/BattleSystem/TBRPG/Combat/Abilties/AC_AbilityComponent.TargActor` _owningabilitycomponent))
  (bind _asbp_pawn_base_player_parent_galypso (cast `/Game/BattleSystem/TBRPG/Combat/CharactersBlueprints/BP_PawnBase_PlayerParent_Galypso` ExecutingActor))
  (`/Game/BattleSystem/TBRPG/Combat/CharactersBlueprints/BP_PawnBase_PlayerParent_Galypso.IlluminateAnim` _asbp_pawn_base_player_parent_galypso)
  (bind _comitted (`self.CommitAbility`))
  (if _comitted
    (bind _component (message `/Game/BattleSystem/TBRPG/Combat/BPI_TurnBasedCombat.GetAbilityComponent` _targactor))
    (bind _output_get (set `self.AbilityEnum` "NewEnumerator2"))
    (`/Game/BattleSystem/TBRPG/Combat/CharactersBlueprints/BP_PawnBase.GetHit` _targactor _output_get)
    (bind _outputdamage (`self.ApplyDefense` _component (`KismetMathLibrary.RandomIntegerInRange` -7 -3)))
    (`/Game/BattleSystem/TBRPG/Combat/Abilties/AC_AbilityComponent.ApplyEffectToTarget` _owningabilitycomponent "NewEnumerator0" _component "LP" "NewEnumerator4" "NewEnumerator0" _outputdamage 0)
    (`/Game/BattleSystem/TBRPG/Combat/Abilties/AC_AbilityComponent.ApplyEffectToTarget` _owningabilitycomponent "NewEnumerator1" _component "BP" "NewEnumerator2" "NewEnumerator1" 0.5 2)
    (`self.EndAbility`)))

(fn `UserConstructionScript`
  (`parent.UserConstructionScript`))