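; BP_TBAbility_StarSear is a turn-based combat ability that damages the owning component's current target.
; On activation and successful commit, it spawns a Niagara effect at the target's location and applies a fixed negative LP effect through the target's ability component.
; It ends after a short delay and prints debug text for success or failed commit.
; The level-based damage scaling nodes are left unconnected.
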(event `self.ActivateAbility`
  (bind _owningabilitycomponent (`self.OwningAbilityComponent`))
  (bind _targactor (`/Game/BattleSystem/TBRPG/Combat/Abilties/AC_AbilityComponent.TargActor` _owningabilitycomponent))
  (bind _comitted (`self.CommitAbility`))
  (if _comitted
    (bind _component (message `/Game/BattleSystem/TBRPG/Combat/BPI_TurnBasedCombat.GetAbilityComponent` _targactor))
    (`NiagaraFunctionLibrary.SpawnSystemAtLocation` (`self.NiagaraSys`) (`self.K2_GetActorLocation` _targactor))
    (`/Game/BattleSystem/TBRPG/Combat/Abilties/AC_AbilityComponent.ApplyEffectToTarget` _owningabilitycomponent "NewEnumerator0" _component "LP" "NewEnumerator4" "NewEnumerator0" -20.0 0)
    (`KismetSystemLibrary.Delay` 2.0)
    (`self.EndAbility`)
    (`KismetSystemLibrary.PrintText` "star sear executed")
    (else
      (`KismetSystemLibrary.PrintText` "star sear not committed"))))

(fn `UserConstructionScript`
  (`parent.UserConstructionScript`))