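; Turn-based RPG combat ability Shadow Cast, performed by the Niren player pawn against the ability component's current target.
; Activation calls Niren's Shadowcast, commits the ability, triggers the target's hit reaction, then applies defense-adjusted damage to LP.
; A coin flip can also apply a randomized one-turn DEF effect and update the target's status.
; Short delays pace the hit and the ability's end.
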(event `self.ActivateAbility`
  (params (ExecutingActor :type "/Game/BattleSystem/TBRPG/Combat/CharactersBlueprints/BP_PawnBase Object Reference"))
  (bind _owningabilitycomponent (`self.OwningAbilityComponent`))
  (bind _targactor (`/Game/BattleSystem/TBRPG/Combat/Abilties/AC_AbilityComponent.TargActor` _owningabilitycomponent))
  (bind _asbp_pawn_base_player_parent_niren (cast `/Game/BattleSystem/TBRPG/Combat/CharactersBlueprints/BP_PawnBase_PlayerParent_Niren` ExecutingActor))
  (`/Game/BattleSystem/TBRPG/Combat/CharactersBlueprints/BP_PawnBase_PlayerParent_Niren.Shadowcast` _asbp_pawn_base_player_parent_niren)
  (bind _comitted (`self.CommitAbility`))
  (if _comitted
    (bind _component (message `/Game/BattleSystem/TBRPG/Combat/BPI_TurnBasedCombat.GetAbilityComponent` _targactor))
    (bind _output_get (set `self.AbilityEnum` "NewEnumerator12"))
    (`/Game/BattleSystem/TBRPG/Combat/CharactersBlueprints/BP_PawnBase.GetHit` _targactor _output_get)
    (`KismetSystemLibrary.Delay` 0.2)
    (bind _outputdamage (`self.ApplyDefense` _component 50))
    (`/Game/BattleSystem/TBRPG/Combat/Abilties/AC_AbilityComponent.ApplyEffectToTarget` _owningabilitycomponent "NewEnumerator0" _component "LP" "NewEnumerator4" "NewEnumerator0" _outputdamage 0)
    (switch `int` (`KismetMathLibrary.RandomIntegerInRange` 0 1)
      (:`0`
        _)
      (:`1`
        (`/Game/BattleSystem/TBRPG/Combat/Abilties/AC_AbilityComponent.ApplyEffectToTarget` _owningabilitycomponent "NewEnumerator1" _component "DEF" "NewEnumerator4" "NewEnumerator0" (`KismetMathLibrary.Conv_IntToDouble` (`KismetMathLibrary.RandomIntegerInRange` 20 35)) 1)
        (set `/Game/BattleSystem/TBRPG/Combat/Abilties/AC_AbilityComponent.CurrentStatus` "NewEnumerator4" _component)
        (`/Game/BattleSystem/TBRPG/Combat/CharactersBlueprints/BP_PawnBase.CheckStatus` _targactor)))
    (`KismetSystemLibrary.Delay` 0.8)
    (`self.EndAbility`)))

(fn `UserConstructionScript`
  (`parent.UserConstructionScript`))