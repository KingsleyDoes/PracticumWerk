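; BP_TBAbility_Shield is a turn-based combat ability that raises the caster's defense.
; Activation requires the executing actor to be the Niren player pawn and the ability to commit.
; It calls the pawn's GetHit with an ability enum, then after a short delay uses AffectSelf on the owning ability component to apply a random-magnitude DEF effect lasting two turns.
; A second short delay precedes EndAbility.
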(event `self.ActivateAbility`
  (params (ExecutingActor :type "/Game/BattleSystem/TBRPG/Combat/CharactersBlueprints/BP_PawnBase Object Reference"))
  (bind _asbp_pawn_base_player_parent_niren (cast `/Game/BattleSystem/TBRPG/Combat/CharactersBlueprints/BP_PawnBase_PlayerParent_Niren` ExecutingActor))
  (`/Game/BattleSystem/TBRPG/Combat/CharactersBlueprints/BP_PawnBase_PlayerParent_Niren.Upcast` _asbp_pawn_base_player_parent_niren)
  (bind _comitted (`self.CommitAbility`))
  (if _comitted
    (bind _output_get (set `self.AbilityEnum` "NewEnumerator11"))
    (`/Game/BattleSystem/TBRPG/Combat/CharactersBlueprints/BP_PawnBase.GetHit` _asbp_pawn_base_player_parent_niren _output_get)
    (`KismetSystemLibrary.Delay` 0.2)
    (`/Game/BattleSystem/TBRPG/Combat/Abilties/AC_AbilityComponent.AffectSelf` (`self.OwningAbilityComponent`) "NewEnumerator1" "DEF" "NewEnumerator5" "NewEnumerator0" (`KismetMathLibrary.Conv_IntToDouble` (`KismetMathLibrary.RandomIntegerInRange` 11 22)) 2)
    (`KismetSystemLibrary.Delay` 0.3)
    (`self.EndAbility`)))

(fn `UserConstructionScript`
  (`parent.UserConstructionScript`))