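; Turn-based RPG ability that weakens the caster's current target and only runs when the executing actor is the Obi player pawn.
; It triggers the pawn's Weaken call, then, if the commit succeeds, sends the target a hit message and applies two timed effects to different stats with differing turn counts.
; It then sets the target's status, has it re-check that status, and ends after a short delay.
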(event `self.ActivateAbility`
  (params (ExecutingActor :type "/Game/BattleSystem/TBRPG/Combat/CharactersBlueprints/BP_PawnBase Object Reference"))
  (bind _owningabilitycomponent (`self.OwningAbilityComponent`))
  (bind _targactor (`/Game/BattleSystem/TBRPG/Combat/Abilties/AC_AbilityComponent.TargActor` _owningabilitycomponent))
  (bind _asbp_pawn_base_player_parent_obi (cast `/Game/BattleSystem/TBRPG/Combat/CharactersBlueprints/BP_PawnBase_PlayerParent_Obi` ExecutingActor))
  (`/Game/BattleSystem/TBRPG/Combat/CharactersBlueprints/BP_PawnBase_PlayerParent_Obi.Weaken` _asbp_pawn_base_player_parent_obi)
  (bind _comitted (`self.CommitAbility`))
  (if _comitted
    (bind _component (message `/Game/BattleSystem/TBRPG/Combat/BPI_TurnBasedCombat.GetAbilityComponent` _targactor))
    (bind _output_get (set `self.AbilityEnum` "NewEnumerator5"))
    (message `/Game/BattleSystem/TBRPG/Combat/BPI_TurnBasedCombat.GetHit` _component _output_get)
    (`/Game/BattleSystem/TBRPG/Combat/Abilties/AC_AbilityComponent.ApplyEffectToTarget` _owningabilitycomponent "NewEnumerator1" _component "LP" "NewEnumerator4" "NewEnumerator1" 0.5 2)
    (`/Game/BattleSystem/TBRPG/Combat/Abilties/AC_AbilityComponent.ApplyEffectToTarget` _owningabilitycomponent "NewEnumerator1" _component "LP" "NewEnumerator2" "NewEnumerator1" 0.5 1)
    (set `/Game/BattleSystem/TBRPG/Combat/Abilties/AC_AbilityComponent.CurrentStatus` "NewEnumerator7" _component)
    (`/Game/BattleSystem/TBRPG/Combat/CharactersBlueprints/BP_PawnBase.CheckStatus` _targactor)
    (`KismetSystemLibrary.Delay` 0.8)
    (`self.EndAbility`)))

(fn `UserConstructionScript`
  (`parent.UserConstructionScript`))