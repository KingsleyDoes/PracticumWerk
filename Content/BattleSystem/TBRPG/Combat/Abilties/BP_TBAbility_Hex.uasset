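; Turn-based RPG combat ability Hex, usable only by the Mushrune enemy pawn.
; On activation it calls the pawn's Hex event, commits the ability, then triggers a hit reaction on the owning ability component's target actor.
; After a short delay it applies a small random negative LP effect through the target's ability component, then ends after another pause.
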(event `self.ActivateAbility`
  (params (ExecutingActor :type "/Game/BattleSystem/TBRPG/Combat/CharactersBlueprints/BP_PawnBase Object Reference"))
  (bind _owningabilitycomponent (`self.OwningAbilityComponent`))
  (bind _targactor (`/Game/BattleSystem/TBRPG/Combat/Abilties/AC_AbilityComponent.TargActor` _owningabilitycomponent))
  (bind _asbp_pawn_base_enemy_parent_mushrune (cast `/Game/BattleSystem/TBRPG/Combat/CharactersBlueprints/Enemies/BP_PawnBase_EnemyParent_Mushrune` ExecutingActor))
  (`/Game/BattleSystem/TBRPG/Combat/CharactersBlueprints/Enemies/BP_PawnBase_EnemyParent_Mushrune.Hex` _asbp_pawn_base_enemy_parent_mushrune)
  (bind _comitted (`self.CommitAbility`))
  (if _comitted
    (bind _component (message `/Game/BattleSystem/TBRPG/Combat/BPI_TurnBasedCombat.GetAbilityComponent` _targactor))
    (bind _output_get (set `self.AbilityEnum` "NewEnumerator1"))
    (`/Game/BattleSystem/TBRPG/Combat/CharactersBlueprints/BP_PawnBase.GetHit` _targactor _output_get)
    (`KismetSystemLibrary.Delay` 0.2)
    (`/Game/BattleSystem/TBRPG/Combat/Abilties/AC_AbilityComponent.ApplyEffectToTarget` _owningabilitycomponent "NewEnumerator0" _component "LP" "NewEnumerator4" "NewEnumerator0" (`KismetMathLibrary.Conv_IntToDouble` (`KismetMathLibrary.RandomIntegerInRange` -7 -3)) 0)
    (`KismetSystemLibrary.Delay` 1.0)
    (`self.EndAbility`)))

(fn `UserConstructionScript`
  (`parent.UserConstructionScript`))