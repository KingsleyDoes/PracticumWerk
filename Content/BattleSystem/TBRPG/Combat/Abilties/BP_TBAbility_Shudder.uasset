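; Turn-based battle ability for the Morchella enemy that debilitates and damages a target.
; On activation it plays the caster's Shudder, commits, triggers the target's hit reaction and disables its ability to act.
; It then reduces BP, applies defense-adjusted LP damage with a damage display, and sets a status on the target.
; Short delays pace the sequence before the ability ends.
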(event `self.ActivateAbility`
  (params (ExecutingActor :type "/Game/BattleSystem/TBRPG/Combat/CharactersBlueprints/BP_PawnBase Object Reference"))
  (bind _owningabilitycomponent (`self.OwningAbilityComponent`))
  (bind _targactor (`/Game/BattleSystem/TBRPG/Combat/Abilties/AC_AbilityComponent.TargActor` _owningabilitycomponent))
  (bind _asbp_pawn_base_enemy_parent_morchella (cast `/Game/BattleSystem/TBRPG/Combat/CharactersBlueprints/Enemies/BP_PawnBase_EnemyParent_Morchella` ExecutingActor))
  (`/Game/BattleSystem/TBRPG/Combat/CharactersBlueprints/Enemies/BP_PawnBase_EnemyParent_Morchella.Shudder` _asbp_pawn_base_enemy_parent_morchella)
  (bind _comitted (`self.CommitAbility`))
  (if _comitted
    (bind _component (message `/Game/BattleSystem/TBRPG/Combat/BPI_TurnBasedCombat.GetAbilityComponent` _targactor))
    (bind _output_get (set `self.AbilityEnum` "NewEnumerator5"))
    (`/Game/BattleSystem/TBRPG/Combat/CharactersBlueprints/BP_PawnBase.GetHit` _targactor _output_get)
    (`KismetSystemLibrary.Delay` 0.2)
    (set `/Game/BattleSystem/TBRPG/Combat/CharactersBlueprints/BP_PawnBase.CanAct` false _targactor)
    (`/Game/BattleSystem/TBRPG/Combat/Abilties/AC_AbilityComponent.ApplyEffectToTarget` _owningabilitycomponent "NewEnumerator0" _component "BP" "NewEnumerator4" "NewEnumerator0" -10.0 1)
    (bind _outputdamage (`self.ApplyDefense` _component -20))
    (`/Game/BattleSystem/TBRPG/Combat/Abilties/AC_AbilityComponent.ApplyEffectToTarget` _owningabilitycomponent "NewEnumerator0" null "LP" "NewEnumerator4" "NewEnumerator0" _outputdamage 1)
    (`/Game/BattleSystem/TBRPG/Combat/CharactersBlueprints/BP_PawnBase.ShowDamage` _targactor (`KismetMathLibrary.FTrunc` _outputdamage))
    (set `/Game/BattleSystem/TBRPG/Combat/Abilties/AC_AbilityComponent.CurrentStatus` "NewEnumerator2" _component)
    (`/Game/BattleSystem/TBRPG/Combat/CharactersBlueprints/BP_PawnBase.CheckStatus` _targactor)
    (`KismetSystemLibrary.Delay` 0.7)
    (`self.EndAbility`)))

(fn `UserConstructionScript`
  (`parent.UserConstructionScript`))