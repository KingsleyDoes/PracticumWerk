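; Turn-based RPG Taunt ability that lowers the DEF of the owning ability component's target.
; Activation casts the executor to the Mehzia player pawn and plays its punch animation before committing.
; On a successful commit, it sends the target a hit tagged with an ability enum.
; After a short delay, it applies a random negative DEF effect through the ability component, then ends the ability.
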(event `self.ActivateAbility`
  (params (ExecutingActor :type "/Game/BattleSystem/TBRPG/Combat/CharactersBlueprints/BP_PawnBase Object Reference"))
  (bind _owningabilitycomponent (`self.OwningAbilityComponent`))
  (bind _targactor (`/Game/BattleSystem/TBRPG/Combat/Abilties/AC_AbilityComponent.TargActor` _owningabilitycomponent))
  (bind _asbp_pawn_base_player_parent_mehzia (cast `/Game/BattleSystem/TBRPG/Combat/CharactersBlueprints/BP_PawnBase_PlayerParent_Mehzia` ExecutingActor))
  (`/Game/BattleSystem/TBRPG/Combat/CharactersBlueprints/BP_PawnBase_PlayerParent_Mehzia.PunchAnimation` _asbp_pawn_base_player_parent_mehzia)
  (bind _comitted (`self.CommitAbility`))
  (if _comitted
    (bind _component (message `/Game/BattleSystem/TBRPG/Combat/BPI_TurnBasedCombat.GetAbilityComponent` _targactor))
    (bind _output_get (set `self.AbilityEnum` "NewEnumerator10"))
    (`/Game/BattleSystem/TBRPG/Combat/CharactersBlueprints/BP_PawnBase.GetHit` _targactor _output_get)
    (`KismetSystemLibrary.Delay` 0.7)
    (`/Game/BattleSystem/TBRPG/Combat/Abilties/AC_AbilityComponent.ApplyEffectToTarget` _owningabilitycomponent "NewEnumerator0" _component "DEF" "NewEnumerator4" "NewEnumerator0" (`KismetMathLibrary.Conv_IntToDouble` (`KismetMathLibrary.RandomIntegerInRange` -8 -2)) 0)
    (`self.EndAbility`)))

(fn `UserConstructionScript`
  (`parent.UserConstructionScript`))