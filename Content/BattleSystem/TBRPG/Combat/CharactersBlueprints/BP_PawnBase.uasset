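; Base combatant pawn for turn-based RPG battles, presenting a character through flipbooks and exposing its ability component.
; BeginPlay randomly nudges Haste, grants the Wait ability and hides the targeting arrow, which targeting later toggles.
; Hits play an effect flipbook chosen by attack name, cleared after a per-attack delay.
; Turn activation refreshes the status icon from the ability component, and PlayDead switches from dying to static death flipbook.
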(event `self.ReceiveBeginPlay`
  (`/Game/BattleSystem/TBRPG/Combat/Abilties/AC_AbilityComponent.AffectSelf` (`self.AC_AbilityComponent`) "NewEnumerator0" "Haste" "NewEnumerator4" "NewEnumerator0" (`KismetMathLibrary.RandomFloatInRange` -2.0 2.0) 0)
  (`/Game/BattleSystem/TBRPG/Combat/Abilties/AC_AbilityComponent.GiveAbility` (`self.AC_AbilityComponent`) "/Game/BattleSystem/TBRPG/Combat/Abilties/BP_TBAbility_Wait.BP_TBAbility_Wait_C")
  (`SceneComponent.SetHiddenInGame` (`self.ArrowSlot`) true false))

(event `/Game/BattleSystem/TBRPG/Combat/BPI_TurnBasedCombat.SetTurnActive`
  (params (IsActive :type Boolean) (HUD :type "/Game/BattleSystem/TBRPG/UI/W_TBBattleHUD Object Reference"))
  (if IsActive
    (`self.CheckStatus`)))

(event `/Game/BattleSystem/TBRPG/Combat/BPI_TurnBasedCombat.SetTargeted`
  (params (IsTargeted :type Boolean))
  (bind _arrowslot (`self.ArrowSlot`))
  (if IsTargeted
    (`SceneComponent.SetHiddenInGame` _arrowslot false false)
    (else
      (`SceneComponent.SetHiddenInGame` _arrowslot true false))))

(event `/Game/BattleSystem/TBRPG/Combat/BPI_TurnBasedCombat.GetHit`
  (params (AttackName :type "/Game/BattleSystem/TBRPG/Combat/Enums/E_AbilityEffectFlipbook Enum" :default "NewEnumerator0"))
  (bind _delaytime (`self.SetEffectAnimation` AttackName))
  (`KismetSystemLibrary.Delay` _delaytime)
  (`self.ResetEffectFlipbook`))

(event `DeadSettle`
  (`KismetSystemLibrary.Delay` 0.4)
  (`PaperFlipbookComponent.SetFlipbook` (`self.Sprite`) (`self.StaticDeathFlipbook`)))

(fn `CheckStatus`
  (bind _statusicon (`self.StatusIcon`))
  (switch `/Game/BattleSystem/TBRPG/Combat/Enums/Enum_Status` (`/Game/BattleSystem/TBRPG/Combat/Abilties/AC_AbilityComponent.CurrentStatus` (`self.AC_AbilityComponent`))
    (:`NewEnumerator0`
      (`PaperFlipbookComponent.SetFlipbook` _statusicon null))
    (:`NewEnumerator1`
      (`PaperFlipbookComponent.SetFlipbook` _statusicon "/Game/BattleSystem/TBRPG/UI/UI_Assets/FBSI_Illuminated.FBSI_Illuminated"))
    (:`NewEnumerator2`
      (`PaperFlipbookComponent.SetFlipbook` _statusicon "/Game/BattleSystem/TBRPG/UI/UI_Assets/FBSI_Hexed.FBSI_Hexed"))
    (:`NewEnumerator3`
      (`PaperFlipbookComponent.SetFlipbook` _statusicon "/Game/BattleSystem/TBRPG/UI/UI_Assets/FBSI_Aura.FBSI_Aura"))
    (:`NewEnumerator4`
      (`PaperFlipbookComponent.SetFlipbook` _statusicon "/Game/BattleSystem/TBRPG/UI/UI_Assets/FBSI_Shadowed.FBSI_Shadowed"))
    (:`NewEnumerator5`
      (`PaperFlipbookComponent.SetFlipbook` _statusicon "/Game/BattleSystem/TBRPG/UI/UI_Assets/FBSI_Shielded.FBSI_Shielded"))
    (:`NewEnumerator6`
      (`PaperFlipbookComponent.SetFlipbook` _statusicon "/Game/BattleSystem/TBRPG/UI/UI_Assets/FBSI_Taunted.FBSI_Taunted"))
    (:`NewEnumerator7`
      (`PaperFlipbookComponent.SetFlipbook` _statusicon "/Game/BattleSystem/TBRPG/UI/UI_Assets/FBSI_Weakened.FBSI_Weakened"))))

(fn `GetAbilityComponent`
  (returns (Component :type "/Game/BattleSystem/TBRPG/Combat/Abilties/AC_AbilityComponent Object Reference"))
  (return (`self.AC_AbilityComponent`)))

(fn `PlayDead`
  (`PaperFlipbookComponent.SetFlipbook` (`self.Sprite`) (`self.DyingFlipbook`))
  (`PaperFlipbookComponent.SetFlipbook` (`self.EffectAnimation`) null)
  (`PaperFlipbookComponent.SetFlipbook` (`self.StatusIcon`) null)
  (`self.DeadSettle`))

(fn `ResetEffectFlipbook`
  (`PaperFlipbookComponent.SetFlipbook` (`self.EffectAnimation`) null))

(fn `ResetFlipbook`
  (`PaperFlipbookComponent.SetFlipbook` (`self.Sprite`) (`self.CombatIdle`)))

(fn `SetEffectAnimation`
  (params (AttackName :type "/Game/BattleSystem/TBRPG/Combat/Enums/E_AbilityEffectFlipbook Enum" :default "NewEnumerator0"))
  (returns (DelayTime :type "Float (double-precision)"))
  (switch `/Game/BattleSystem/TBRPG/Combat/Enums/E_AbilityEffectFlipbook` AttackName
    (:`NewEnumerator0`
      (`PaperFlipbookComponent.SetFlipbook` (`self.EffectAnimation`) "/Game/BattleSystem/TBRPG/PixelAssets/EffectArt/Flipbooks/FBE_Punch.FBE_Punch")
      (return 0.6))
    (:`NewEnumerator1`
      (`PaperFlipbookComponent.SetFlipbook` (`self.EffectAnimation`) "/Game/BattleSystem/TBRPG/PixelAssets/EffectArt/Flipbooks/FBE_Rend.FBE_Rend")
      (return 0.9))
    (:`NewEnumerator2`
      (`PaperFlipbookComponent.SetFlipbook` (`self.EffectAnimation`) "/Game/BattleSystem/TBRPG/PixelAssets/EffectArt/Flipbooks/FBE_Illuminate.FBE_Illuminate")
      (`PaperFlipbookComponent.SetFlipbook` (`self.StatusIcon`) null)
      (return 0.7))
    (:`NewEnumerator3`
      (`PaperFlipbookComponent.SetFlipbook` (`self.EffectAnimation`) "/Game/BattleSystem/TBRPG/PixelAssets/EffectArt/Flipbooks/FBE_Uplift.FBE_Uplift")
      (return 0.6))
    (:`NewEnumerator4`
      (`PaperFlipbookComponent.SetFlipbook` (`self.EffectAnimation`) "/Game/BattleSystem/TBRPG/PixelAssets/EffectArt/Flipbooks/FBE_SpikeRain.FBE_SpikeRain")
      (return 0.9))
    (:`NewEnumerator5`
      (`PaperFlipbookComponent.SetFlipbook` (`self.EffectAnimation`) "/Game/BattleSystem/TBRPG/PixelAssets/EffectArt/Flipbooks/FBE_Trickmatize.FBE_Trickmatize")
      (return 0.8))
    (:`NewEnumerator6`
      (`PaperFlipbookComponent.SetFlipbook` (`self.EffectAnimation`) "/Game/BattleSystem/TBRPG/PixelAssets/EffectArt/Flipbooks/FBE_HeartBurst.FBE_HeartBurst")
      (return 1.1))
    (:`NewEnumerator7`
      (`PaperFlipbookComponent.SetFlipbook` (`self.EffectAnimation`) "/Game/BattleSystem/TBRPG/PixelAssets/EffectArt/Flipbooks/FB_Replenish.FB_Replenish")
      (return 1.0))
    (:`NewEnumerator8`
      (`PaperFlipbookComponent.SetFlipbook` (`self.EffectAnimation`) "/Game/BattleSystem/TBRPG/PixelAssets/EffectArt/Flipbooks/FB_SingleSpike.FB_SingleSpike")
      (return 0.7))
    (:`NewEnumerator9`
      (`PaperFlipbookComponent.SetFlipbook` (`self.EffectAnimation`) "/Game/BattleSystem/TBRPG/PixelAssets/EffectArt/Flipbooks/FB_StarSear.FB_StarSear")
      (return 1.1))
    (:`NewEnumerator10`
      (`PaperFlipbookComponent.SetFlipbook` (`self.EffectAnimation`) "/Game/BattleSystem/TBRPG/PixelAssets/EffectArt/Flipbooks/FB_Gust.FB_Gust")
      (return 0.7))
    (:`NewEnumerator11`
      (`PaperFlipbookComponent.SetFlipbook` (`self.EffectAnimation`) "/Game/BattleSystem/TBRPG/PixelAssets/EffectArt/Flipbooks/FB_Shield.FB_Shield")
      (return 0.9))
    (:`NewEnumerator12`
      (`PaperFlipbookComponent.SetFlipbook` (`self.EffectAnimation`) "/Game/BattleSystem/TBRPG/PixelAssets/EffectArt/Flipbooks/FB_Swirl.FB_Swirl")
      (return 0.9))
    (:`NewEnumerator13`
      (`PaperFlipbookComponent.SetFlipbook` (`self.EffectAnimation`) "/Game/BattleSystem/TBRPG/PixelAssets/EffectArt/Flipbooks/FB_Putdown.FB_Putdown")
      (return 0.6))
    (:`NewEnumerator14`
      (`PaperFlipbookComponent.SetFlipbook` (`self.EffectAnimation`) "/Game/BattleSystem/TBRPG/PixelAssets/EffectArt/Flipbooks/FB_ClodHit.FB_ClodHit")
      (return 0.9))))

(fn `UserConstructionScript`)