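; Turn-based combat pawn for the Mushrune enemy, setting its name, idle and death flipbooks, and granting Wait and Trickmatize abilities on BeginPlay.
; On an active turn it checks status, always activates Wait, shows the ability banner on the HUD, then ends the turn.
; Trickmatize is never chosen here; its event shares Ruminate's brief attack flipbook animation before resetting.
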(event `self.ReceiveBeginPlay`
  (bind _ac_abilitycomponent (`self.AC_AbilityComponent`))
  (`parent.ReceiveBeginPlay`)
  (`/Game/BattleSystem/TBRPG/Combat/Abilties/AC_AbilityComponent.GiveAbility` _ac_abilitycomponent "/Game/BattleSystem/TBRPG/Combat/Abilties/BP_TBAbility_Wait.BP_TBAbility_Wait_C")
  (`/Game/BattleSystem/TBRPG/Combat/Abilties/AC_AbilityComponent.GiveAbility` _ac_abilitycomponent "/Game/BattleSystem/TBRPG/Combat/Abilties/BP_TBAbility_Trickmatize.BP_TBAbility_Trickmatize_C")
  (set `self.CombatIdle` "/Game/BattleSystem/TBRPG/PixelAssets/EnemyArt/FB_MushruneIdle.FB_MushruneIdle")
  (set `self.DisplayName` "Mushrune")
  (set `self.DyingFlipbook` "/Game/BattleSystem/TBRPG/PixelAssets/EnemyArt/FBD_Mushrune.FBD_Mushrune")
  (set `self.StaticDeathFlipbook` "/Game/BattleSystem/TBRPG/PixelAssets/EnemyArt/FBDS_Mushrune.FBDS_Mushrune"))

(event `Ruminate`
  (`PaperFlipbookComponent.SetFlipbook` (`self.Sprite`) "/Game/BattleSystem/TBRPG/PixelAssets/EnemyArt/FB_MushruneAttack.FB_MushruneAttack" :!label _label)
  (`KismetSystemLibrary.Delay` 0.9)
  (`self.ResetFlipbook`))

(event `Trickmatize`
  (goto _label))

(event `self.SetTurnActive`
  (params (IsActive :type Boolean) (HUD :type "/Game/BattleSystem/TBRPG/UI/W_TBBattleHUD Object Reference"))
  (bind _ac_abilitycomponent (`self.AC_AbilityComponent`))
  (if IsActive
    (`self.CheckStatus`)
    (`/Game/BattleSystem/TBRPG/Combat/Abilties/AC_AbilityComponent.StartTurn` _ac_abilitycomponent)
    (`KismetSystemLibrary.Delay` 0.1)
    (bind _returnedability (`/Game/BattleSystem/TBRPG/Combat/Abilties/AC_AbilityComponent.ActivateOwnedAbility` :`self` _ac_abilitycomponent :`AbilityClass` "/Game/BattleSystem/TBRPG/Combat/Abilties/BP_TBAbility_Wait.BP_TBAbility_Wait_C"))
    (`KismetSystemLibrary.PrintText` "clodder waited" true true (struct :`R` 0.63797 :`G` 1.0 :`A` 1.0) 5.0)
    (`/Game/BattleSystem/TBRPG/UI/W_TBBattleHUD.AbilityUsedBannerText` HUD self (`/Game/BattleSystem/TBRPG/Combat/Abilties/BP_TBAbility.Name` _returnedability))
    (`KismetSystemLibrary.Delay` 0.2)
    (`/Game/BattleSystem/TBRPG/Combat/Abilties/AC_AbilityComponent.EndTurn` _ac_abilitycomponent _returnedability)))

(fn `UserConstructionScript`
  (`parent.UserConstructionScript`))