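; Sporemonger enemy pawn for the turn-based RPG combat system, built on the enemy parent pawn.
; BeginPlay sets its flipbooks, name and Lifesteal, Burst and Infection abilities, then applies a random Haste penalty to itself.
; Turn start runs its StateTree, while SetTurnActive starts the turn and ends it after a delay if still active.
; Each ability event shows a banner, plays an action flipbook, then resets and ends the turn.
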(event `self.ReceiveBeginPlay`
  (`parent.ReceiveBeginPlay`)
  (set `self.CombatIdle` "/Game/BattleSystem/TBRPG/PixelAssets/EnemyArt/FB_Sporemonger-Idle.FB_Sporemonger-Idle")
  (set `self.DisplayName` "Sporemonger")
  (set `self.DyingFlipbook` "/Game/BattleSystem/TBRPG/PixelAssets/EnemyArt/FBD_Sporemonger.FBD_Sporemonger")
  (set `self.StaticDeathFlipbook` "/Game/BattleSystem/TBRPG/PixelAssets/EnemyArt/FBDS_Sporemonger.FBDS_Sporemonger")
  (set `self.EnemyAbilities` (`|MakeArray` "/Game/BattleSystem/TBRPG/Combat/Abilties/BP_TBAbility_Lifesteal.BP_TBAbility_Lifesteal_C" "/Game/BattleSystem/TBRPG/Combat/Abilties/BP_TBAbility_Burst.BP_TBAbility_Burst_C" "/Game/BattleSystem/TBRPG/Combat/Abilties/BP_TBAbility_Infection.BP_TBAbility_Infection_C" :!type "/Game/BattleSystem/TBRPG/Combat/Abilties/BP_TBAbility Class Reference"))
  (set `self.Dead` false)
  (`/Game/BattleSystem/TBRPG/Combat/Abilties/AC_AbilityComponent.AffectSelf` (`self.AC_AbilityComponent`) "NewEnumerator0" "Haste" "NewEnumerator4" "NewEnumerator0" (`KismetMathLibrary.RandomFloatInRange` -5.0 -1.0) 0))

(event `self.AC_AbilityComponent.TurnStarted`
  (`BrainComponent.StartLogic` (`self.StateTree`)))

(event `self.SetTurnActive`
  (params (IsActive :type Boolean) (HUD :type "/Game/BattleSystem/TBRPG/UI/W_TBBattleHUD Object Reference"))
  (if IsActive
    (`self.CheckStatus`)
    (`/Game/BattleSystem/TBRPG/Combat/Abilties/AC_AbilityComponent.StartTurn` (`self.AC_AbilityComponent`))
    (`KismetSystemLibrary.Delay` 3.0)
    (if IsActive
      (`/Game/BattleSystem/TBRPG/Combat/Abilties/AC_AbilityComponent.EndTurn` (`self.AC_AbilityComponent`) null))))

(event `Infection`
  (`/Game/BattleSystem/TBRPG/UI/W_TBBattleHUD.AbilityUsedBannerText` (stale `self.SetTurnActive` HUD) self "Infection")
  (`PaperFlipbookComponent.SetFlipbook` (`self.Sprite`) "/Game/BattleSystem/TBRPG/PixelAssets/EnemyArt/FB_Sporemonger-Action.FB_Sporemonger-Action" :!label _label)
  (`KismetSystemLibrary.Delay` 0.4 :!label _label_2)
  (`self.ResetFlipbook`)
  (`/Game/BattleSystem/TBRPG/Combat/Abilties/AC_AbilityComponent.EndTurn` (`self.AC_AbilityComponent`) null))

(event `Burst`
  (`/Game/BattleSystem/TBRPG/UI/W_TBBattleHUD.AbilityUsedBannerText` (stale `self.SetTurnActive` HUD) self "Burst")
  (goto _label))

(event `Lifesteal`
  (`/Game/BattleSystem/TBRPG/UI/W_TBBattleHUD.AbilityUsedBannerText` (stale `self.SetTurnActive` HUD) self "Lifesteal")
  (`PaperFlipbookComponent.SetFlipbook` (`self.Sprite`) "/Game/BattleSystem/TBRPG/PixelAssets/EnemyArt/FB_Sporemonger-Lifesteal.FB_Sporemonger-Lifesteal")
  (goto _label_2))

(fn `UserConstructionScript`
  (`parent.UserConstructionScript`))