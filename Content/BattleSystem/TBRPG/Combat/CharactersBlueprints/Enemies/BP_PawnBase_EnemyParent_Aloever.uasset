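; Aloever enemy pawn for turn-based RPG combat, configured on BeginPlay with its flipbooks, name and three abilities: Prickle, Slap and Replenish.
; An active turn checks status and starts the ability component's turn, whose TurnStarted event restarts the StateTree logic.
; Ability events (Sploosh displays as Replenish) show a HUD banner, then share one delayed sequence that plays the attack flipbook, resets it and ends the turn.
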(event `self.ReceiveBeginPlay`
  (`parent.ReceiveBeginPlay`)
  (set `self.CombatIdle` "/Game/BattleSystem/TBRPG/PixelAssets/EnemyArt/FB_AloeverIdle.FB_AloeverIdle")
  (set `self.DisplayName` "Aloever")
  (set `self.DyingFlipbook` "/Game/BattleSystem/TBRPG/PixelAssets/EnemyArt/FBD_Aloever.FBD_Aloever")
  (set `self.StaticDeathFlipbook` "/Game/BattleSystem/TBRPG/PixelAssets/EnemyArt/FBDS_Aloever.FBDS_Aloever")
  (set `self.EnemyAbilities` (`|MakeArray` "/Game/BattleSystem/TBRPG/Combat/Abilties/BP_TBAbility_Prickle.BP_TBAbility_Prickle_C" "/Game/BattleSystem/TBRPG/Combat/Abilties/BP_TBAbility_Slap.BP_TBAbility_Slap_C" "/Game/BattleSystem/TBRPG/Combat/Abilties/BP_TBAbility_Replenish.BP_TBAbility_Replenish_C" :!type "/Game/BattleSystem/TBRPG/Combat/Abilties/BP_TBAbility Class Reference"))
  (set `self.Dead` false))

(event `self.SetTurnActive`
  (params (IsActive :type Boolean) (HUD :type "/Game/BattleSystem/TBRPG/UI/W_TBBattleHUD Object Reference"))
  (if IsActive
    (`self.CheckStatus`)
    (`/Game/BattleSystem/TBRPG/Combat/Abilties/AC_AbilityComponent.StartTurn` (`self.AC_AbilityComponent`))))

(event `self.AC_AbilityComponent.TurnStarted`
  (`BrainComponent.RestartLogic` (`self.StateTree`)))

(event `Sploosh`
  (`/Game/BattleSystem/TBRPG/UI/W_TBBattleHUD.AbilityUsedBannerText` (stale `self.SetTurnActive` HUD) self "Replenish")
  (`PaperFlipbookComponent.SetFlipbook` (`self.Sprite`) "/Game/BattleSystem/TBRPG/PixelAssets/EnemyArt/FB_AloeverAttack.FB_AloeverAttack" :!label _label)
  (`KismetSystemLibrary.Delay` 1.4)
  (`self.ResetFlipbook`)
  (`KismetSystemLibrary.Delay` 5.0)
  (`/Game/BattleSystem/TBRPG/Combat/Abilties/AC_AbilityComponent.EndTurn` (`self.AC_AbilityComponent`) null))

(event `Prickle`
  (`/Game/BattleSystem/TBRPG/UI/W_TBBattleHUD.AbilityUsedBannerText` (stale `self.SetTurnActive` HUD) self "Prickle")
  (goto _label))

(event `Slap`
  (`/Game/BattleSystem/TBRPG/UI/W_TBBattleHUD.AbilityUsedBannerText` (stale `self.SetTurnActive` HUD) self "Slap")
  (goto _label))

(fn `UserConstructionScript`
  (`parent.UserConstructionScript`))