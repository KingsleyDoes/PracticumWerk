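; Enemy pawn for Hittake in the turn-based RPG combat, built on the shared enemy parent.
; BeginPlay sets its name, idle and death flipbooks, and three abilities: Mega Spore Blast, Spore Blast and Umbral Shield.
; Becoming active checks status and starts the ability component's turn, which restarts the StateTree logic.
; Each ability event shows a HUD banner, plays timed flipbook animations, then resets the sprite and ends the turn.
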(event `self.ReceiveBeginPlay`
  (`parent.ReceiveBeginPlay`)
  (set `self.CombatIdle` "/Game/BattleSystem/TBRPG/PixelAssets/EnemyArt/FB_HittakeIdle.FB_HittakeIdle")
  (set `self.DisplayName` "Hittake")
  (set `self.DyingFlipbook` "/Game/BattleSystem/TBRPG/PixelAssets/EnemyArt/FBD_HittakeIdle.FBD_HittakeIdle")
  (set `self.StaticDeathFlipbook` "/Game/BattleSystem/TBRPG/PixelAssets/EnemyArt/FBDS_HittakeIdle.FBDS_HittakeIdle")
  (set `self.EnemyAbilities` (`|MakeArray` "/Game/BattleSystem/TBRPG/Combat/Abilties/BP_TBAbility_MegaSporeBlast.BP_TBAbility_MegaSporeBlast_C" "/Game/BattleSystem/TBRPG/Combat/Abilties/BP_TBAbility_SporeBlast.BP_TBAbility_SporeBlast_C" "/Game/BattleSystem/TBRPG/Combat/Abilties/BP_TBAbility_UmbralShield.BP_TBAbility_UmbralShield_C" :!type "/Game/BattleSystem/TBRPG/Combat/Abilties/BP_TBAbility Class Reference"))
  (set `self.Dead` false))

(event `self.SetTurnActive`
  (params (IsActive :type Boolean) (HUD :type "/Game/BattleSystem/TBRPG/UI/W_TBBattleHUD Object Reference"))
  (if IsActive
    (`self.CheckStatus`)
    (`/Game/BattleSystem/TBRPG/Combat/Abilties/AC_AbilityComponent.StartTurn` (`self.AC_AbilityComponent`))))

(event `self.AC_AbilityComponent.TurnStarted`
  (`BrainComponent.RestartLogic` (`self.StateTree`)))

(event `SporeBlast`
  (`/Game/BattleSystem/TBRPG/UI/W_TBBattleHUD.AbilityUsedBannerText` (stale `self.SetTurnActive` HUD) self "Spore Blast")
  (`PaperFlipbookComponent.SetFlipbook` (`self.Sprite`) "/Game/BattleSystem/TBRPG/PixelAssets/EnemyArt/FB_HittakeShoot.FB_HittakeShoot" :!label _label)
  (`KismetSystemLibrary.Delay` 1.9)
  (`self.ResetFlipbook` :!label _label_2)
  (`KismetSystemLibrary.Delay` 1.0)
  (`/Game/BattleSystem/TBRPG/Combat/Abilties/AC_AbilityComponent.EndTurn` (`self.AC_AbilityComponent`) null))

(event `MegaSporeBlast`
  (`/Game/BattleSystem/TBRPG/UI/W_TBBattleHUD.AbilityUsedBannerText` (stale `self.SetTurnActive` HUD) self "Mega Spore Blast")
  (goto _label))

(event `UmbralShield`
  (bind _sprite (`self.Sprite`))
  (`/Game/BattleSystem/TBRPG/UI/W_TBBattleHUD.AbilityUsedBannerText` (stale `self.SetTurnActive` HUD) self "Umbral Shield")
  (`PaperFlipbookComponent.SetFlipbook` _sprite "/Game/BattleSystem/TBRPG/PixelAssets/EnemyArt/FB_HittakeShoot.FB_HittakeShoot")
  (`KismetSystemLibrary.Delay` 0.7)
  (`PaperFlipbookComponent.SetFlipbook` _sprite "/Game/BattleSystem/TBRPG/PixelAssets/EnemyArt/FB_HittakeDefendIdle.FB_HittakeDefendIdle")
  (`KismetSystemLibrary.Delay` 0.8)
  (`PaperFlipbookComponent.SetFlipbook` _sprite "/Game/BattleSystem/TBRPG/PixelAssets/EnemyArt/FB_HittakeExitDefent.FB_HittakeExitDefent")
  (`KismetSystemLibrary.Delay` 0.7)
  (goto _label_2))

(fn `UserConstructionScript`
  (`parent.UserConstructionScript`))