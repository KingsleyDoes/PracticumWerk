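; Cractus enemy pawn for the turn-based RPG combat, setting its flipbooks, name and three spike-themed abilities on BeginPlay, plus a random negative Haste adjustment.
; An active turn checks status, then starts through the ability component or ends immediately if unable to act, with a delayed EndTurn as fallback.
; TurnStarted runs the StateTree logic.
; Each ability event shows its banner, then shares one attack flipbook sequence that ends the turn.
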(event `self.ReceiveBeginPlay`
  (`parent.ReceiveBeginPlay`)
  (set `self.CombatIdle` "/Game/BattleSystem/TBRPG/PixelAssets/EnemyArt/FB_CractusIdle.FB_CractusIdle")
  (set `self.DisplayName` "Cractus")
  (set `self.DyingFlipbook` "/Game/BattleSystem/TBRPG/PixelAssets/EnemyArt/FBD_Cractus.FBD_Cractus")
  (set `self.StaticDeathFlipbook` "/Game/BattleSystem/TBRPG/PixelAssets/EnemyArt/FBDS_Cractus.FBDS_Cractus")
  (set `self.EnemyAbilities` (`|MakeArray` "/Game/BattleSystem/TBRPG/Combat/Abilties/BP_TBAbility_SpikeRain.BP_TBAbility_SpikeRain_C" "/Game/BattleSystem/TBRPG/Combat/Abilties/BP_TBAbility_SpikeToss.BP_TBAbility_SpikeToss_C" "/Game/BattleSystem/TBRPG/Combat/Abilties/BP_TBAbility_Acupuncture.BP_TBAbility_Acupuncture_C" :!type "/Game/BattleSystem/TBRPG/Combat/Abilties/BP_TBAbility Class Reference"))
  (set `self.Dead` false)
  (`/Game/BattleSystem/TBRPG/Combat/Abilties/AC_AbilityComponent.AffectSelf` (`self.AC_AbilityComponent`) "NewEnumerator0" "Haste" "NewEnumerator4" "NewEnumerator0" (`KismetMathLibrary.RandomFloatInRange` -5.0 -1.0) 0))

(event `self.AC_AbilityComponent.TurnStarted`
  (`BrainComponent.StartLogic` (`self.StateTree`)))

(event `self.SetTurnActive`
  (params (IsActive :type Boolean) (HUD :type "/Game/BattleSystem/TBRPG/UI/W_TBBattleHUD Object Reference"))
  (bind _ac_abilitycomponent (`self.AC_AbilityComponent`))
  (if IsActive
    (`self.CheckStatus`)
    (if (`self.CanAct`)
      (`/Game/BattleSystem/TBRPG/Combat/Abilties/AC_AbilityComponent.StartTurn` _ac_abilitycomponent)
      (`KismetSystemLibrary.Delay` 4.0)
      (if IsActive
        (`/Game/BattleSystem/TBRPG/Combat/Abilties/AC_AbilityComponent.EndTurn` (`self.AC_AbilityComponent`) null))
      (else
        (`/Game/BattleSystem/TBRPG/Combat/Abilties/AC_AbilityComponent.EndTurn` _ac_abilitycomponent null)))))

(event `SpikeRain`
  (`/Game/BattleSystem/TBRPG/UI/W_TBBattleHUD.AbilityUsedBannerText` (stale `self.SetTurnActive` HUD) self "Spike Rain")
  (`PaperFlipbookComponent.SetFlipbook` (`self.Sprite`) "/Game/BattleSystem/TBRPG/PixelAssets/EnemyArt/FB_CractusAttack.FB_CractusAttack" :!label _label)
  (`KismetSystemLibrary.Delay` 0.7)
  (`self.ResetFlipbook`)
  (`/Game/BattleSystem/TBRPG/Combat/Abilties/AC_AbilityComponent.EndTurn` (`self.AC_AbilityComponent`) null))

(event `Acupuncture`
  (`/Game/BattleSystem/TBRPG/UI/W_TBBattleHUD.AbilityUsedBannerText` (stale `self.SetTurnActive` HUD) self "Acupuncture")
  (goto _label))

(event `Spike Toss`
  (`/Game/BattleSystem/TBRPG/UI/W_TBBattleHUD.AbilityUsedBannerText` (stale `self.SetTurnActive` HUD) self "Spike Toss")
  (goto _label))

(fn `UserConstructionScript`
  (`parent.UserConstructionScript`))