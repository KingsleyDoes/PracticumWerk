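; Captain enemy pawn for turn-based combat, configured on BeginPlay with Cractus idle and death flipbooks and three abilities: Vanquishing Blow, Beat and Resurge.
; An active turn checks status and starts the ability component's turn, whose TurnStarted event launches StateTree logic.
; Each ability event shows its HUD banner, then shares one sequence: attack flipbook, short delay, flipbook reset and turn end.
; These events apply no damage or effects themselves.
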(event `self.ReceiveBeginPlay`
  (`parent.ReceiveBeginPlay`)
  (set `self.CombatIdle` "/Game/BattleSystem/TBRPG/PixelAssets/EnemyArt/FB_CractusIdle.FB_CractusIdle")
  (set `self.DisplayName` "Captain")
  (set `self.DyingFlipbook` "/Game/BattleSystem/TBRPG/PixelAssets/EnemyArt/FBD_Cractus.FBD_Cractus")
  (set `self.StaticDeathFlipbook` "/Game/BattleSystem/TBRPG/PixelAssets/EnemyArt/FBDS_Cractus.FBDS_Cractus")
  (set `self.EnemyAbilities` (`|MakeArray` "/Game/BattleSystem/TBRPG/Combat/Abilties/BP_TBAbility_VanquishingBlow.BP_TBAbility_VanquishingBlow_C" "/Game/BattleSystem/TBRPG/Combat/Abilties/BP_TBAbility_Beat.BP_TBAbility_Beat_C" "/Game/BattleSystem/TBRPG/Combat/Abilties/BP_TBAbility_Resurge.BP_TBAbility_Resurge_C" :!type "/Game/BattleSystem/TBRPG/Combat/Abilties/BP_TBAbility Class Reference"))
  (set `self.Dead` false))

(event `self.SetTurnActive`
  (params (IsActive :type Boolean) (HUD :type "/Game/BattleSystem/TBRPG/UI/W_TBBattleHUD Object Reference"))
  (if IsActive
    (`self.CheckStatus`)
    (`/Game/BattleSystem/TBRPG/Combat/Abilties/AC_AbilityComponent.StartTurn` (`self.AC_AbilityComponent`))))

(event `self.AC_AbilityComponent.TurnStarted`
  (`BrainComponent.StartLogic` (`self.StateTree`)))

(event `Resurge`
  (`/Game/BattleSystem/TBRPG/UI/W_TBBattleHUD.AbilityUsedBannerText` (stale `self.SetTurnActive` HUD) self "Resurge")
  (`PaperFlipbookComponent.SetFlipbook` (`self.Sprite`) "/Game/BattleSystem/TBRPG/PixelAssets/EnemyArt/FB_CractusAttack.FB_CractusAttack" :!label _label)
  (`KismetSystemLibrary.Delay` 0.7)
  (`self.ResetFlipbook`)
  (`/Game/BattleSystem/TBRPG/Combat/Abilties/AC_AbilityComponent.EndTurn` (`self.AC_AbilityComponent`) null))

(event `Beat`
  (`/Game/BattleSystem/TBRPG/UI/W_TBBattleHUD.AbilityUsedBannerText` (stale `self.SetTurnActive` HUD) self "Beat")
  (goto _label))

(event `Vanquishing Blow`
  (`/Game/BattleSystem/TBRPG/UI/W_TBBattleHUD.AbilityUsedBannerText` (stale `self.SetTurnActive` HUD) self "Vanquishing Blow")
  (goto _label))

(fn `UserConstructionScript`
  (`parent.UserConstructionScript`))