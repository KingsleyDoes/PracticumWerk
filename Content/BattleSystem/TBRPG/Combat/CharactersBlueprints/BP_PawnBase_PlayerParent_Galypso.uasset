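; Player combat pawn for Galypso in the turn-based RPG battle system, using Paper2D flipbooks for its states.
; BeginPlay reads the saved character level to grant abilities cumulatively, while SetStatsFromLevel and CamraderieStatBoost set level-scaled stats and LP/BP boosts.
; SetTurnActive runs turn visuals and a delay-based timeout, or skips the turn when unable to act.
; Ability animation events show a banner, share one attack sequence, then end the turn.
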(event `self.ReceiveBeginPlay`
  (bind _ac_abilitycomponent (`self.AC_AbilityComponent`))
  (`parent.ReceiveBeginPlay`)
  (`|ExecutionSequence`
    (:`then_0`
      (bind _asgi_custom_game_instance (cast `/Game/BattleSystem/TBRPG/SaveSystem/GI_CustomGameInstance` (`GameplayStatics.GetGameInstance`)))
      (bind _savedata (`/Game/BattleSystem/TBRPG/SaveSystem/BPI_SaveInterface.GetGameData` _asgi_custom_game_instance))
      (bind (_playersavestruct_levelscompleted _playersavestruct_characterlevel) (break `/Game/BattleSystem/TBRPG/SaveSystem/S_PlayerSave` (`/Game/BattleSystem/TBRPG/SaveSystem/SG_SaveSystem.PlayerSaveStruct` _savedata)))
      (switch `int` _playersavestruct_characterlevel
        (:`Default`
          _)
        (:`0`
          _)
        (:`1`
          (`/Game/BattleSystem/TBRPG/Combat/Abilties/AC_AbilityComponent.GiveAbility` _ac_abilitycomponent "/Game/BattleSystem/TBRPG/Combat/Abilties/BP_TBAbility_Illuminate.BP_TBAbility_Illuminate_C" :!label _label))
        (:`2`
          (`/Game/BattleSystem/TBRPG/Combat/Abilties/AC_AbilityComponent.GiveAbility` _ac_abilitycomponent "/Game/BattleSystem/TBRPG/Combat/Abilties/BP_TBAbility_Dazzle.BP_TBAbility_Dazzle_C" :!label _label_2)
          (goto _label))
        (:`3`
          (`/Game/BattleSystem/TBRPG/Combat/Abilties/AC_AbilityComponent.GiveAbility` _ac_abilitycomponent "/Game/BattleSystem/TBRPG/Combat/Abilties/BP_TBAbility_StarSear.BP_TBAbility_StarSear_C" :!label _label_3)
          (goto _label_2))
        (:`4`
          (`/Game/BattleSystem/TBRPG/Combat/Abilties/AC_AbilityComponent.GiveAbility` _ac_abilitycomponent "/Game/BattleSystem/TBRPG/Combat/Abilties/BP_TBAbility_MegaAura.BP_TBAbility_MegaAura_C")
          (goto _label_3)))
      (`/Game/BattleSystem/TBRPG/Combat/Abilties/AC_AbilityComponent.GiveAbility` _ac_abilitycomponent "/Game/BattleSystem/TBRPG/Combat/Abilties/BP_TBAbility_Wait.BP_TBAbility_Wait_C"))
    (:`then_1`
      (set `self.DyingFlipbook` "/Game/BattleSystem/TBRPG/PixelAssets/CharacterArt/galypso/FBD_Galypso.FBD_Galypso")
      (set `self.CanAct` true)
      (set `self.CombatIdle` "/Game/BattleSystem/TBRPG/PixelAssets/CharacterArt/galypso/FB_GalypsoIdle.FB_GalypsoIdle")
      (set `self.StaticDeathFlipbook` "/Game/BattleSystem/TBRPG/PixelAssets/CharacterArt/galypso/FBDS_Galypso.FBDS_Galypso"))))

(event `IlluminateAnim`
  (`self.BannerAbilityFill` self "Illuminate")
  (`PaperFlipbookComponent.SetFlipbook` (`self.Sprite`) "/Game/BattleSystem/TBRPG/PixelAssets/CharacterArt/galypso/FB_GalypsoAttack.FB_GalypsoAttack" :!label _label_4)
  (`KismetSystemLibrary.Delay` 1.0)
  (`self.ResetFlipbook`)
  (`KismetSystemLibrary.Delay` 0.75)
  (`/Game/BattleSystem/TBRPG/Combat/Abilties/AC_AbilityComponent.EndTurn` (`self.AC_AbilityComponent`) null))

(event `/Game/BattleSystem/TBRPG/Combat/BPI_TurnBasedCombat.SetTurnActive`
  (params (IsActive :type Boolean) (HUD :type "/Game/BattleSystem/TBRPG/UI/W_TBBattleHUD Object Reference"))
  (bind _sprite (`self.Sprite`))
  (if (`self.CanAct`)
    (if IsActive
      (`|ExecutionSequence`
        (:`then_0`
          (`self.CheckStatus`)
          (`PaperFlipbookComponent.SetFlipbook` _sprite "/Game/BattleSystem/TBRPG/PixelAssets/CharacterArt/galypso/FB_Galypso_Activate.FB_Galypso_Activate")
          (`KismetSystemLibrary.Delay` 1.1)
          (`PaperFlipbookComponent.SetFlipbook` _sprite "/Game/BattleSystem/TBRPG/PixelAssets/CharacterArt/galypso/FB_GalypsoCombatIdle.FB_GalypsoCombatIdle")
          (`SceneComponent.SetHiddenInGame` (`self.ArrowSlot`) false false))
        (:`then_1`
          (`KismetSystemLibrary.Delay` 12.0)
          (if IsActive
            (`self.TimeRanOut`)
            (`/Game/BattleSystem/TBRPG/Combat/Abilties/AC_AbilityComponent.EndTurn` (`self.AC_AbilityComponent`) null))))
      (else
        (`PaperFlipbookComponent.SetFlipbook` _sprite "/Game/BattleSystem/TBRPG/PixelAssets/CharacterArt/galypso/FB_GalypsoIdle.FB_GalypsoIdle")))
    (elif IsActive
      (`KismetSystemLibrary.PrintText` "can't act" true true (struct :`R` 0.214583 :`B` 0.05113 :`A` 1.0) 5.0)
      (`KismetSystemLibrary.Delay` 2.0)
      (`/Game/BattleSystem/TBRPG/UI/W_TBBattleHUD.ClearUI` HUD)
      (`/Game/BattleSystem/TBRPG/Combat/Abilties/AC_AbilityComponent.EndTurn` (`self.AC_AbilityComponent`) null))))

(event `StarSearAnim`
  (`self.BannerAbilityFill` self "Star Sear")
  (goto _label_4))

(event `MegaAuraAnim`
  (`self.BannerAbilityFill` null "Mega Aura")
  (goto _label_4))

(event `DazzleAnim`
  (`self.BannerAbilityFill` null "Dazzle")
  (goto _label_4))

(event `/Game/BattleSystem/TBRPG/Combat/BPI_TurnBasedCombat.CamraderieStatBoost`
  (bind _ac_abilitycomponent (`self.AC_AbilityComponent`))
  (bind _camboost (`self.CamBoost`))
  (bind _savedata (message `/Game/BattleSystem/TBRPG/SaveSystem/BPI_SaveInterface.GetGameData` (`GameplayStatics.GetGameInstance`)))
  (bind (_playersavestruct_levelscompleted _playersavestruct_characterlevel) (break `/Game/BattleSystem/TBRPG/SaveSystem/S_PlayerSave` (`/Game/BattleSystem/TBRPG/SaveSystem/SG_SaveSystem.PlayerSaveStruct` _savedata)))
  (switch `int` _playersavestruct_characterlevel
    (:`1`
      (set `self.CamBoost` 5.0))
    (:`2`
      (set `self.CamBoost` 10.0))
    (:`3`
      (set `self.CamBoost` 15.0))
    (:`4`
      (set `self.CamBoost` 25.0)))
  (`/Game/BattleSystem/TBRPG/Combat/Abilties/AC_AbilityComponent.AffectSelf` _ac_abilitycomponent "NewEnumerator0" "LP" "NewEnumerator5" "NewEnumerator0" _camboost 0)
  (`/Game/BattleSystem/TBRPG/Combat/Abilties/AC_AbilityComponent.AffectSelf` _ac_abilitycomponent "NewEnumerator0" "BP" "NewEnumerator5" "NewEnumerator0" _camboost 0)
  (set `self.IsBoosted` true))

(event `Wait`
  (`PaperFlipbookComponent.SetFlipbook` (`self.Sprite`) "/Game/BattleSystem/TBRPG/PixelAssets/CharacterArt/galypso/FB_Galypso_Deactivate.FB_Galypso_Deactivate")
  (`KismetSystemLibrary.Delay` 0.7)
  (`self.ResetFlipbook`)
  (`KismetSystemLibrary.Delay` 0.1)
  (`/Game/BattleSystem/TBRPG/Combat/Abilties/AC_AbilityComponent.EndTurn` (`self.AC_AbilityComponent`) null))

(fn `SetStatsFromLevel`
  (params (Level :type Integer))
  (locals (`LV-LP` :type "Float (double-precision)") (`LV-BP` :type "Float (double-precision)") (`LV-HS` :type "Float (double-precision)") (`LV-DF` :type "Float (double-precision)"))
  (bind _lv_lp (`local.LV-LP`))
  (bind _lv_bp (`local.LV-BP`))
  (bind _lv_hs (`local.LV-HS`))
  (bind _lv_df (`local.LV-DF`))
  (switch `int` Level
    (:`1`
      ; Setting local variables
      (set `local.LV-LP` 35.0)
      (set `local.LV-BP` 35.0)
      (set `local.LV-HS` 20.0)
      (set `local.LV-DF` 15.0)
      ;[0.0444 0.15 0 0.5] Life
      (`self.SetStat` "LP" "NewEnumerator4" _lv_lp)
      (`self.SetStat` "LP" "NewEnumerator2" _lv_lp)
      ;[0 0.1434 0.15 0.5] Breath
      (`self.SetStat` "BP" "NewEnumerator4" _lv_bp)
      (`self.SetStat` "BP" "NewEnumerator2" _lv_bp)
      ;[0.15 0.1353 0 0.5] Haste
      (`self.SetStat` "Haste" "NewEnumerator4" _lv_hs)
      ;[0 0.02524 0.15 0.5] Defense
      (`self.SetStat` "DEF" "NewEnumerator4" _lv_df))
    (:`2`
      (set `local.LV-LP` 45.0)
      (set `local.LV-BP` 45.0)
      (set `local.LV-HS` 30.0)
      (set `local.LV-DF` 25.0)
      (`self.SetStat` "LP" "NewEnumerator4" _lv_lp)
      (`self.SetStat` "LP" "NewEnumerator2" _lv_lp)
      (`self.SetStat` "BP" "NewEnumerator4" _lv_bp)
      (`self.SetStat` "BP" "NewEnumerator2" _lv_bp)
      (`self.SetStat` "Haste" "NewEnumerator4" _lv_hs)
      (`self.SetStat` "DEF" "NewEnumerator4" _lv_df))
    (:`3`
      (set `local.LV-LP` 55.0)
      (set `local.LV-BP` 55.0)
      (set `local.LV-HS` 40.0)
      (set `local.LV-DF` 35.0)
      (`self.SetStat` "LP" "NewEnumerator4" _lv_lp)
      (`self.SetStat` "LP" "NewEnumerator2" _lv_lp)
      (`self.SetStat` "BP" "NewEnumerator4" _lv_bp)
      (`self.SetStat` "BP" "NewEnumerator2" _lv_bp)
      (`self.SetStat` "Haste" "NewEnumerator4" _lv_hs)
      (`self.SetStat` "DEF" "NewEnumerator4" _lv_df))
    (:`4`
      (set `local.LV-LP` 70.0)
      (set `local.LV-BP` 70.0)
      (set `local.LV-HS` 60.0)
      (set `local.LV-DF` 50.0)
      (`self.SetStat` "LP" "NewEnumerator4" _lv_lp)
      (`self.SetStat` "LP" "NewEnumerator2" _lv_lp)
      (`self.SetStat` "BP" "NewEnumerator4" _lv_bp)
      (`self.SetStat` "BP" "NewEnumerator2" _lv_bp)
      (`self.SetStat` "Haste" "NewEnumerator4" _lv_hs)
      (`self.SetStat` "DEF" "NewEnumerator4" _lv_df))))

(fn `UserConstructionScript`
  (`parent.UserConstructionScript`))