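; Niren's player pawn for turn-based RPG combat, handling its abilities, sprite animations and turn flow.
; On BeginPlay it reads the saved character level and grants abilities through a fall-through switch, so levels up to four stack unlocks on Wait; other values get only Wait.
; Turn activation checks status and swaps flipbooks, or shows a skip banner and ends the turn when unable to act.
; Upcast and Rend events play timed animations, then end the turn.
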(event `self.ReceiveBeginPlay`
  (bind _ac_abilitycomponent (`self.AC_AbilityComponent`))
  (`parent.ReceiveBeginPlay`)
  (`|ExecutionSequence`
    (:`then_0`
      (bind _asgi_custom_game_instance (cast `/Game/BattleSystem/TBRPG/SaveSystem/GI_CustomGameInstance` (`GameplayStatics.GetGameInstance`)))
      (bind _savedata (`/Game/BattleSystem/TBRPG/SaveSystem/BPI_SaveInterface.GetGameData` _asgi_custom_game_instance))
      (bind (_playersavestruct_levelscompleted _playersavestruct_characterlevel) (break `/Game/BattleSystem/TBRPG/SaveSystem/S_PlayerSave` (`/Game/BattleSystem/TBRPG/SaveSystem/SG_SaveSystem.PlayerSaveStruct` _savedata)))
      (switch `int` _playersavestruct_characterlevel
        (:`Default`
          _)
        (:`0`
          _)
        (:`1`
          (`/Game/BattleSystem/TBRPG/Combat/Abilties/AC_AbilityComponent.GiveAbility` _ac_abilitycomponent "/Game/BattleSystem/TBRPG/Combat/Abilties/BP_TBAbility_Rend.BP_TBAbility_Rend_C" :!label _label))
        (:`2`
          (`/Game/BattleSystem/TBRPG/Combat/Abilties/AC_AbilityComponent.GiveAbility` _ac_abilitycomponent "/Game/BattleSystem/TBRPG/Combat/Abilties/BP_TBAbility_Shield.BP_TBAbility_Shield_C" :!label _label_2)
          (goto _label))
        (:`3`
          (`/Game/BattleSystem/TBRPG/Combat/Abilties/AC_AbilityComponent.GiveAbility` _ac_abilitycomponent "/Game/BattleSystem/TBRPG/Combat/Abilties/BP_TBAbility_ForceWave.BP_TBAbility_ForceWave_C" :!label _label_3)
          (goto _label_2))
        (:`4`
          (`/Game/BattleSystem/TBRPG/Combat/Abilties/AC_AbilityComponent.GiveAbility` _ac_abilitycomponent "/Game/BattleSystem/TBRPG/Combat/Abilties/BP_TBAbility_ShadowCast.BP_TBAbility_ShadowCast_C")
          (goto _label_3)))
      (`/Game/BattleSystem/TBRPG/Combat/Abilties/AC_AbilityComponent.GiveAbility` _ac_abilitycomponent "/Game/BattleSystem/TBRPG/Combat/Abilties/BP_TBAbility_Wait.BP_TBAbility_Wait_C"))
    (:`then_1`
      (set `self.CombatIdle` "/Game/BattleSystem/TBRPG/PixelAssets/CharacterArt/niren/niren-testsprite-idle1.niren-testsprite-idle1")
      (set `self.CanAct` true)
      (set `self.StaticDeathFlipbook` "/Game/BattleSystem/TBRPG/PixelAssets/CharacterArt/niren/FBDS_Niren.FBDS_Niren"))))

(event `Upcast`
  (`PaperFlipbookComponent.SetFlipbook` (`self.Sprite`) "/Game/BattleSystem/TBRPG/PixelAssets/CharacterArt/niren/FB_NirenUpcast.FB_NirenUpcast")
  (`KismetSystemLibrary.Delay` 0.5)
  (`self.ResetFlipbook`)
  (`/Game/BattleSystem/TBRPG/Combat/Abilties/AC_AbilityComponent.EndTurn` (`self.AC_AbilityComponent`) null))

(event `Rend`
  (`PaperFlipbookComponent.SetFlipbook` (`self.Sprite`) "/Game/BattleSystem/TBRPG/PixelAssets/CharacterArt/niren/FB_NirenAttack.FB_NirenAttack")
  (`KismetSystemLibrary.Delay` 1.0)
  (`self.ResetFlipbook`)
  (`/Game/BattleSystem/TBRPG/Combat/Abilties/AC_AbilityComponent.EndTurn` (`self.AC_AbilityComponent`) null))

(event `/Game/BattleSystem/TBRPG/Combat/BPI_TurnBasedCombat.SetTurnActive`
  (params (IsActive :type Boolean) (HUD :type "/Game/BattleSystem/TBRPG/UI/W_TBBattleHUD Object Reference"))
  (bind _sprite (`self.Sprite`))
  (if (`self.CanAct`)
    (if IsActive
      (`self.CheckStatus`)
      (`PaperFlipbookComponent.SetFlipbook` _sprite "/Game/BattleSystem/TBRPG/PixelAssets/CharacterArt/niren/niren-testsprite-action.niren-testsprite-action")
      (`KismetSystemLibrary.Delay` 0.7)
      (`PaperFlipbookComponent.SetFlipbook` _sprite "/Game/BattleSystem/TBRPG/PixelAssets/CharacterArt/niren/niren-testsprite-Combatidle.niren-testsprite-Combatidle")
      (else
        (`PaperFlipbookComponent.SetFlipbook` _sprite "/Game/BattleSystem/TBRPG/PixelAssets/CharacterArt/niren/niren-testsprite-idle1.niren-testsprite-idle1")))
    (else
      (`/Game/BattleSystem/TBRPG/UI/W_TBBattleHUD.TurnSkipBannerText` HUD self)
      (`KismetSystemLibrary.Delay` 1.0)
      (`/Game/BattleSystem/TBRPG/UI/W_TBBattleHUD.ClearUI` HUD)
      (`/Game/BattleSystem/TBRPG/Combat/Abilties/AC_AbilityComponent.EndTurn` (`self.AC_AbilityComponent`) null))))

(fn `UserConstructionScript`
  (`parent.UserConstructionScript`))