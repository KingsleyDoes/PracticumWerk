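; Player party pawn for Obi in turn-based RPG combat, a child of the player pawn base that sets his flipbooks, stats and abilities.
; BeginPlay reads the saved character level and grants Wait plus a cumulative set of support abilities through the ability component.
; Turn and ability events play flipbooks with timed delays, then end the turn; an Obi unable to act auto-activates Wait.
; Level switches also set base stats and scale the camaraderie LP/BP boost.
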(event `self.ReceiveBeginPlay`
  (bind _ac_abilitycomponent (`self.AC_AbilityComponent`))
  (`parent.ReceiveBeginPlay`)
  (`|ExecutionSequence`
    (:`then_0`
      (bind _asgi_custom_game_instance (cast `/Game/BattleSystem/TBRPG/SaveSystem/GI_CustomGameInstance` (`GameplayStatics.GetGameInstance`)))
      (bind _savedata (`/Game/BattleSystem/TBRPG/SaveSystem/BPI_SaveInterface.GetGameData` _asgi_custom_game_instance))
      (bind (_playersavestruct_levelscompleted _playersavestruct_characterlevel) (break `/Game/BattleSystem/TBRPG/SaveSystem/S_PlayerSave` (`/Game/BattleSystem/TBRPG/SaveSystem/SG_SaveSystem.PlayerSaveStruct` _savedata)))
      (switch `int` _playersavestruct_characterlevel
        (:`Default`
          _)
        (:`0`
          _)
        (:`1`
          (`/Game/BattleSystem/TBRPG/Combat/Abilties/AC_AbilityComponent.GiveAbility` _ac_abilitycomponent "/Game/BattleSystem/TBRPG/Combat/Abilties/BP_TBAbility_Uplift.BP_TBAbility_Uplift_C" :!label _label))
        (:`2`
          (`/Game/BattleSystem/TBRPG/Combat/Abilties/AC_AbilityComponent.GiveAbility` _ac_abilitycomponent "/Game/BattleSystem/TBRPG/Combat/Abilties/BP_TBAbility_Mend.BP_TBAbility_Mend_C" :!label _label_2)
          (goto _label))
        (:`3`
          (`/Game/BattleSystem/TBRPG/Combat/Abilties/AC_AbilityComponent.GiveAbility` _ac_abilitycomponent "/Game/BattleSystem/TBRPG/Combat/Abilties/BP_TBAbility_Weaken.BP_TBAbility_Weaken_C" :!label _label_3)
          (goto _label_2))
        (:`4`
          (`/Game/BattleSystem/TBRPG/Combat/Abilties/AC_AbilityComponent.GiveAbility` _ac_abilitycomponent "/Game/BattleSystem/TBRPG/Combat/Abilties/BP_TBAbility_Inspire.BP_TBAbility_Inspire_C")
          (goto _label_3)))
      (`/Game/BattleSystem/TBRPG/Combat/Abilties/AC_AbilityComponent.GiveAbility` _ac_abilitycomponent "/Game/BattleSystem/TBRPG/Combat/Abilties/BP_TBAbility_Wait.BP_TBAbility_Wait_C"))
    (:`then_1`
      (set `self.CombatIdle` "/Game/BattleSystem/TBRPG/PixelAssets/CharacterArt/obi/FB_ObiIdle.FB_ObiIdle")
      (set `self.CanAct` true)
      (set `self.StaticDeathFlipbook` "/Game/BattleSystem/TBRPG/PixelAssets/CharacterArt/obi/FBDS_Obi.FBDS_Obi")
      (set `self.DyingFlipbook` "/Game/BattleSystem/TBRPG/PixelAssets/CharacterArt/obi/FBD_Obi.FBD_Obi"))))

(event `Wait`
  (`PaperFlipbookComponent.SetFlipbook` (`self.Sprite`) "/Game/BattleSystem/TBRPG/PixelAssets/CharacterArt/obi/FB_Obi_Deactivate.FB_Obi_Deactivate")
  (`KismetSystemLibrary.Delay` 0.4)
  (`self.ResetFlipbook`)
  (`KismetSystemLibrary.Delay` 0.1)
  (`/Game/BattleSystem/TBRPG/Combat/Abilties/AC_AbilityComponent.EndTurn` (`self.AC_AbilityComponent`) null))

(event `/Game/BattleSystem/TBRPG/Combat/BPI_TurnBasedCombat.SetTurnActive`
  (params (IsActive :type Boolean) (HUD :type "/Game/BattleSystem/TBRPG/UI/W_TBBattleHUD Object Reference"))
  (bind _sprite (`self.Sprite`))
  (if (`self.CanAct`)
    (if IsActive
      (`PaperFlipbookComponent.SetFlipbook` _sprite "/Game/BattleSystem/TBRPG/PixelAssets/CharacterArt/obi/FB_Obi_Activate.FB_Obi_Activate")
      (`KismetSystemLibrary.Delay` 0.4)
      (`PaperFlipbookComponent.SetFlipbook` _sprite "/Game/BattleSystem/TBRPG/PixelAssets/CharacterArt/obi/FB_Obi_CombatIdle.FB_Obi_CombatIdle")
      (`KismetSystemLibrary.Delay` 0.6)
      (`SceneComponent.SetHiddenInGame` (`self.ArrowSlot`) false false)
      (else
        (`PaperFlipbookComponent.SetFlipbook` _sprite "/Game/BattleSystem/TBRPG/PixelAssets/CharacterArt/obi/FB_ObiIdle.FB_ObiIdle")))
    (else
      (`/Game/BattleSystem/TBRPG/UI/W_TBBattleHUD.TurnSkipBannerText` HUD self)
      (`KismetSystemLibrary.Delay` 1.0)
      (`/Game/BattleSystem/TBRPG/Combat/Abilties/AC_AbilityComponent.ActivateOwnedAbility` :`self` (`self.AC_AbilityComponent`) :`AbilityClass` "/Game/BattleSystem/TBRPG/Combat/Abilties/BP_TBAbility_Wait.BP_TBAbility_Wait_C"))))

(event `Inspire`
  (`self.BannerAbilityFill` null "Inspire")
  (`PaperFlipbookComponent.SetFlipbook` (`self.Sprite`) "/Game/BattleSystem/TBRPG/PixelAssets/CharacterArt/obi/FB_Obi_Action.FB_Obi_Action" :!label _label_4)
  (`KismetSystemLibrary.Delay` 0.8)
  (`self.ResetFlipbook`)
  (`KismetSystemLibrary.Delay` 0.95)
  (`/Game/BattleSystem/TBRPG/Combat/Abilties/AC_AbilityComponent.EndTurn` (`self.AC_AbilityComponent`) null))

(event `Mend`
  (`self.BannerAbilityFill` null "Mend")
  (goto _label_4))

(event `Weaken`
  (`self.BannerAbilityFill` null "Weaken")
  (goto _label_4))

(event `Uplift`
  (`self.BannerAbilityFill` null "Uplift")
  (goto _label_4))

(event `/Game/BattleSystem/TBRPG/Combat/BPI_TurnBasedCombat.CamraderieStatBoost`
  (bind _camboost (`self.CamBoost`))
  (bind _ac_abilitycomponent (`self.AC_AbilityComponent`))
  (bind _savedata (message `/Game/BattleSystem/TBRPG/SaveSystem/BPI_SaveInterface.GetGameData` (`GameplayStatics.GetGameInstance`)))
  (bind (_playersavestruct_levelscompleted _playersavestruct_characterlevel) (break `/Game/BattleSystem/TBRPG/SaveSystem/S_PlayerSave` (`/Game/BattleSystem/TBRPG/SaveSystem/SG_SaveSystem.PlayerSaveStruct` _savedata)))
  (switch `int` _playersavestruct_characterlevel
    (:`1`
      (set `self.CamBoost` 5.0))
    (:`2`
      (set `self.CamBoost` 10.0))
    (:`3`
      (set `self.CamBoost` 15.0))
    (:`4`
      (set `self.CamBoost` 25.0)))
  (`/Game/BattleSystem/TBRPG/Combat/Abilties/AC_AbilityComponent.AffectSelf` _ac_abilitycomponent "NewEnumerator0" "LP" "NewEnumerator5" "NewEnumerator0" _camboost 0)
  (`/Game/BattleSystem/TBRPG/Combat/Abilties/AC_AbilityComponent.AffectSelf` _ac_abilitycomponent "NewEnumerator0" "BP" "NewEnumerator5" "NewEnumerator0" _camboost 0)
  (set `self.IsBoosted` true))

(fn `SetStatsFromLevel`
  (params (Level :type Integer))
  (locals (`LV-LP` :type "Float (double-precision)") (`LV-BP` :type "Float (double-precision)") (`LV-HS` :type "Float (double-precision)") (`LV-DF` :type "Float (double-precision)"))
  (bind _lv_lp (`local.LV-LP`))
  (bind _lv_bp (`local.LV-BP`))
  (bind _lv_hs (`local.LV-HS`))
  (bind _lv_df (`local.LV-DF`))
  (switch `int` Level
    (:`1`
      ; Setting local variables
      (set `local.LV-LP` 35.0)
      (set `local.LV-BP` 35.0)
      (set `local.LV-HS` 1.0)
      (set `local.LV-DF` 10.0)
      ;[0.0444 0.15 0 0.5] Life
      (`self.SetStat` "LP" "NewEnumerator4" _lv_lp)
      (`self.SetStat` "LP" "NewEnumerator2" _lv_lp)
      ;[0 0.1434 0.15 0.5] Breath
      (`self.SetStat` "BP" "NewEnumerator4" _lv_bp)
      (`self.SetStat` "BP" "NewEnumerator2" _lv_bp)
      ;[0.15 0.1353 0 0.5] Haste
      (`self.SetStat` "Haste" "NewEnumerator4" _lv_hs)
      ;[0 0.02524 0.15 0.5] Defense
      (`self.SetStat` "DEF" "NewEnumerator4" _lv_df))
    (:`2`
      (set `local.LV-LP` 45.0)
      (set `local.LV-BP` 45.0)
      (set `local.LV-HS` 2.0)
      (set `local.LV-DF` 15.0)
      (`self.SetStat` "LP" "NewEnumerator4" _lv_lp)
      (`self.SetStat` "LP" "NewEnumerator2" _lv_lp)
      (`self.SetStat` "BP" "NewEnumerator4" _lv_bp)
      (`self.SetStat` "BP" "NewEnumerator2" _lv_bp)
      (`self.SetStat` "Haste" "NewEnumerator4" _lv_hs)
      (`self.SetStat` "DEF" "NewEnumerator4" _lv_df))
    (:`3`
      (set `local.LV-LP` 55.0)
      (set `local.LV-BP` 55.0)
      (set `local.LV-HS` 3.0)
      (set `local.LV-DF` 20.0)
      (`self.SetStat` "LP" "NewEnumerator4" _lv_lp)
      (`self.SetStat` "LP" "NewEnumerator2" _lv_lp)
      (`self.SetStat` "BP" "NewEnumerator4" _lv_bp)
      (`self.SetStat` "BP" "NewEnumerator2" _lv_bp)
      (`self.SetStat` "Haste" "NewEnumerator4" _lv_hs)
      (`self.SetStat` "DEF" "NewEnumerator4" _lv_df))
    (:`4`
      (set `local.LV-LP` 70.0)
      (set `local.LV-BP` 70.0)
      (set `local.LV-HS` 4.0)
      (set `local.LV-DF` 25.0)
      (`self.SetStat` "LP" "NewEnumerator4" _lv_lp)
      (`self.SetStat` "LP" "NewEnumerator2" _lv_lp)
      (`self.SetStat` "BP" "NewEnumerator4" _lv_bp)
      (`self.SetStat` "BP" "NewEnumerator2" _lv_bp)
      (`self.SetStat` "Haste" "NewEnumerator4" _lv_hs)
      (`self.SetStat` "DEF" "NewEnumerator4" _lv_df))))

(fn `UserConstructionScript`
  (`parent.UserConstructionScript`))