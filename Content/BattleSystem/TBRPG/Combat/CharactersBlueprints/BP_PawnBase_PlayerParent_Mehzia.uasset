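; Player combat pawn for Mehzia in the turn-based battle system, a child of the player parent pawn.
; BeginPlay reads the saved character level to grant abilities cumulatively and sets her flipbooks.
; Ability events play a banner and sprite animation, then end the turn through the ability component.
; SetTurnActive enforces a turn timeout or skips turns when unable to act, while level tables drive stats and camaraderie boosts.
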(event `self.ReceiveBeginPlay`
  (bind _ac_abilitycomponent (`self.AC_AbilityComponent`))
  (`parent.ReceiveBeginPlay`)
  (`|ExecutionSequence`
    (:`then_0`
      (bind _asgi_custom_game_instance (cast `/Game/BattleSystem/TBRPG/SaveSystem/GI_CustomGameInstance` (`GameplayStatics.GetGameInstance`)))
      (bind _savedata (`/Game/BattleSystem/TBRPG/SaveSystem/BPI_SaveInterface.GetGameData` _asgi_custom_game_instance))
      (bind (_playersavestruct_levelscompleted _playersavestruct_characterlevel) (break `/Game/BattleSystem/TBRPG/SaveSystem/S_PlayerSave` (`/Game/BattleSystem/TBRPG/SaveSystem/SG_SaveSystem.PlayerSaveStruct` _savedata)))
      (switch `int` _playersavestruct_characterlevel
        (:`Default`
          _)
        (:`0`
          _)
        (:`1`
          (`/Game/BattleSystem/TBRPG/Combat/Abilties/AC_AbilityComponent.GiveAbility` _ac_abilitycomponent "/Game/BattleSystem/TBRPG/Combat/Abilties/BP_TBAbility_Punch.BP_TBAbility_Punch_C" :!label _label))
        (:`2`
          (`/Game/BattleSystem/TBRPG/Combat/Abilties/AC_AbilityComponent.GiveAbility` _ac_abilitycomponent "/Game/BattleSystem/TBRPG/Combat/Abilties/BP_TBAbility_PowerfulBlow.BP_TBAbility_PowerfulBlow_C" :!label _label_2)
          (goto _label))
        (:`3`
          (`/Game/BattleSystem/TBRPG/Combat/Abilties/AC_AbilityComponent.GiveAbility` _ac_abilitycomponent "/Game/BattleSystem/TBRPG/Combat/Abilties/BP_TBAbility_Taunt.BP_TBAbility_Taunt_C" :!label _label_3)
          (goto _label_2))
        (:`4`
          (`/Game/BattleSystem/TBRPG/Combat/Abilties/AC_AbilityComponent.GiveAbility` _ac_abilitycomponent "/Game/BattleSystem/TBRPG/Combat/Abilties/BP_TBAbility_BurnDefense.BP_TBAbility_BurnDefense_C")
          (goto _label_3)))
      (`/Game/BattleSystem/TBRPG/Combat/Abilties/AC_AbilityComponent.GiveAbility` _ac_abilitycomponent "/Game/BattleSystem/TBRPG/Combat/Abilties/BP_TBAbility_Wait.BP_TBAbility_Wait_C"))
    (:`then_1`
      (set `self.DyingFlipbook` "/Game/BattleSystem/TBRPG/PixelAssets/CharacterArt/Mehzia/FBD_Mehzia.FBD_Mehzia")
      (set `self.CombatIdle` "/Game/BattleSystem/TBRPG/PixelAssets/CharacterArt/Mehzia/FB_MehziaIdle.FB_MehziaIdle")
      (set `self.CanAct` true)
      (set `self.StaticDeathFlipbook` "/Game/BattleSystem/TBRPG/PixelAssets/CharacterArt/Mehzia/FBDS_Mehzia.FBDS_Mehzia"))))

(event `PunchAnimation`
  (`self.BannerAbilityFill` self "Punch")
  (`PaperFlipbookComponent.SetFlipbook` (`self.Sprite`) "/Game/BattleSystem/TBRPG/PixelAssets/CharacterArt/Mehzia/FB_MehziaPunch.FB_MehziaPunch")
  (`KismetSystemLibrary.Delay` 0.7)
  (`self.ResetFlipbook`)
  (`KismetSystemLibrary.Delay` 1.05)
  (`/Game/BattleSystem/TBRPG/Combat/Abilties/AC_AbilityComponent.EndTurn` (`self.AC_AbilityComponent`) null))

(event `PowerfulBlow`
  (`self.BannerAbilityFill` self "Powerful Blow")
  (`PaperFlipbookComponent.SetFlipbook` (`self.Sprite`) "/Game/BattleSystem/TBRPG/PixelAssets/CharacterArt/Mehzia/FB_MehziaDoublePunch.FB_MehziaDoublePunch")
  (`KismetSystemLibrary.Delay` 0.8)
  (`self.ResetFlipbook`)
  (`KismetSystemLibrary.Delay` 0.95)
  (`/Game/BattleSystem/TBRPG/Combat/Abilties/AC_AbilityComponent.EndTurn` (`self.AC_AbilityComponent`) null :!label _label_4))

(event `/Game/BattleSystem/TBRPG/Combat/BPI_TurnBasedCombat.SetTurnActive`
  (params (IsActive :type Boolean) (HUD :type "/Game/BattleSystem/TBRPG/UI/W_TBBattleHUD Object Reference"))
  (if IsActive
    (`self.CheckStatus`)
    (if (`self.CanAct`)
      (`|ExecutionSequence`
        (:`then_0`
          (`PaperFlipbookComponent.SetFlipbook` (`self.Sprite`) "/Game/BattleSystem/TBRPG/PixelAssets/CharacterArt/Mehzia/FB_MehziaCombatIdle.FB_MehziaCombatIdle")
          (`KismetSystemLibrary.Delay` 1.0)
          (`SceneComponent.SetHiddenInGame` (`self.ArrowSlot`) false false))
        (:`then_1`
          (`KismetSystemLibrary.Delay` 12.0)
          (if IsActive
            (`self.TimeRanOut`)
            (`/Game/BattleSystem/TBRPG/Combat/Abilties/AC_AbilityComponent.EndTurn` (`self.AC_AbilityComponent`) null))))
      (else
        (`KismetSystemLibrary.PrintText` "can't act" true true (struct :`R` 0.214583 :`B` 0.05113 :`A` 1.0) 5.0)
        (`KismetSystemLibrary.Delay` 2.0)
        (`/Game/BattleSystem/TBRPG/UI/W_TBBattleHUD.ClearUI` HUD)
        (`/Game/BattleSystem/TBRPG/Combat/Abilties/AC_AbilityComponent.EndTurn` (`self.AC_AbilityComponent`) null)
        (`KismetSystemLibrary.Delay` 3.0)
        (if IsActive
          (`self.TimeRanOut`)
          (`/Game/BattleSystem/TBRPG/Combat/Abilties/AC_AbilityComponent.EndTurn` (`self.AC_AbilityComponent`) null))))
    (else
      (`PaperFlipbookComponent.SetFlipbook` (`self.Sprite`) "/Game/BattleSystem/TBRPG/PixelAssets/CharacterArt/Mehzia/FB_MehziaIdle.FB_MehziaIdle"))))

(event `Taunt`
  (`self.BannerAbilityFill` self "Taunt")
  (`PaperFlipbookComponent.SetFlipbook` (`self.Sprite`) "/Game/BattleSystem/TBRPG/PixelAssets/CharacterArt/Mehzia/FB_MehziaTaunt.FB_MehziaTaunt" :!label _label_5)
  (`KismetSystemLibrary.Delay` 0.6)
  (`self.ResetFlipbook`)
  (`KismetSystemLibrary.Delay` 1.15)
  (goto _label_4))

(event `BurnDefense`
  (`self.BannerAbilityFill` self "Burn Defense")
  (goto _label_5))

(event `Wait`
  (`self.ResetFlipbook`)
  (`KismetSystemLibrary.Delay` 0.1)
  (`/Game/BattleSystem/TBRPG/Combat/Abilties/AC_AbilityComponent.EndTurn` (`self.AC_AbilityComponent`) null))

(event `/Game/BattleSystem/TBRPG/Combat/BPI_TurnBasedCombat.CamraderieStatBoost`
  (bind _camboost (`self.CamBoost`))
  (bind _ac_abilitycomponent (`self.AC_AbilityComponent`))
  (bind _savedata (message `/Game/BattleSystem/TBRPG/SaveSystem/BPI_SaveInterface.GetGameData` (`GameplayStatics.GetGameInstance`)))
  (bind (_playersavestruct_levelscompleted _playersavestruct_characterlevel) (break `/Game/BattleSystem/TBRPG/SaveSystem/S_PlayerSave` (`/Game/BattleSystem/TBRPG/SaveSystem/SG_SaveSystem.PlayerSaveStruct` _savedata)))
  (switch `int` _playersavestruct_characterlevel
    (:`1`
      (set `self.CamBoost` 5.0))
    (:`2`
      (set `self.CamBoost` 10.0))
    (:`3`
      (set `self.CamBoost` 15.0))
    (:`4`
      (set `self.CamBoost` 25.0)))
  (`/Game/BattleSystem/TBRPG/Combat/Abilties/AC_AbilityComponent.AffectSelf` _ac_abilitycomponent "NewEnumerator0" "LP" "NewEnumerator5" "NewEnumerator0" _camboost 0)
  (`/Game/BattleSystem/TBRPG/Combat/Abilties/AC_AbilityComponent.AffectSelf` _ac_abilitycomponent "NewEnumerator0" "BP" "NewEnumerator5" "NewEnumerator0" _camboost 0)
  (set `self.IsBoosted` true))

(fn `SetStatsFromLevel`
  (params (Level :type Integer))
  (locals (`LV-LP` :type "Float (double-precision)") (`LV-BP` :type "Float (double-precision)") (`LV-HS` :type "Float (double-precision)") (`LV-DF` :type "Float (double-precision)"))
  (bind _lv_lp (`local.LV-LP`))
  (bind _lv_bp (`local.LV-BP`))
  (bind _lv_hs (`local.LV-HS`))
  (bind _lv_df (`local.LV-DF`))
  (switch `int` Level
    (:`1`
      ; Setting local variables
      (set `local.LV-LP` 50.0)
      (set `local.LV-BP` 25.0)
      (set `local.LV-HS` 30.0)
      (set `local.LV-DF` 25.0)
      ;[0.0444 0.15 0 0.5] Life
      (`self.SetStat` "LP" "NewEnumerator4" _lv_lp)
      (`self.SetStat` "LP" "NewEnumerator2" _lv_lp)
      ;[0 0.1434 0.15 0.5] Breath
      (`self.SetStat` "BP" "NewEnumerator4" _lv_bp)
      (`self.SetStat` "BP" "NewEnumerator2" _lv_bp)
      ;[0.15 0.1353 0 0.5] Haste
      (`self.SetStat` "Haste" "NewEnumerator4" _lv_hs)
      ;[0 0.02524 0.15 0.5] Defense
      (`self.SetStat` "DEF" "NewEnumerator4" _lv_df))
    (:`2`
      (set `local.LV-LP` 60.0)
      (set `local.LV-BP` 35.0)
      (set `local.LV-HS` 50.0)
      (set `local.LV-DF` 30.0)
      (`self.SetStat` "LP" "NewEnumerator4" _lv_lp)
      (`self.SetStat` "LP" "NewEnumerator2" _lv_lp)
      (`self.SetStat` "BP" "NewEnumerator4" _lv_bp)
      (`self.SetStat` "BP" "NewEnumerator2" _lv_bp)
      (`self.SetStat` "Haste" "NewEnumerator4" _lv_hs)
      (`self.SetStat` "DEF" "NewEnumerator4" _lv_df))
    (:`3`
      (set `local.LV-LP` 70.0)
      (set `local.LV-BP` 45.0)
      (set `local.LV-HS` 70.0)
      (set `local.LV-DF` 40.0)
      (`self.SetStat` "LP" "NewEnumerator4" _lv_lp)
      (`self.SetStat` "LP" "NewEnumerator2" _lv_lp)
      (`self.SetStat` "BP" "NewEnumerator4" _lv_bp)
      (`self.SetStat` "BP" "NewEnumerator2" _lv_bp)
      (`self.SetStat` "Haste" "NewEnumerator4" _lv_hs)
      (`self.SetStat` "DEF" "NewEnumerator4" _lv_df))
    (:`4`
      (set `local.LV-LP` 90.0)
      (set `local.LV-BP` 60.0)
      (set `local.LV-HS` 90.0)
      (set `local.LV-DF` 50.0)
      (`self.SetStat` "LP" "NewEnumerator4" _lv_lp)
      (`self.SetStat` "LP" "NewEnumerator2" _lv_lp)
      (`self.SetStat` "BP" "NewEnumerator4" _lv_bp)
      (`self.SetStat` "BP" "NewEnumerator2" _lv_bp)
      (`self.SetStat` "Haste" "NewEnumerator4" _lv_hs)
      (`self.SetStat` "DEF" "NewEnumerator4" _lv_df))))

(fn `UserConstructionScript`
  (`parent.UserConstructionScript`))