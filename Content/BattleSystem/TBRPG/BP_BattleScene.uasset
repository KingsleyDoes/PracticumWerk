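; Turn-based RPG battle scene pawn that stages the player's party and spawns enemy encounters.
; StartBattle stores the return pawn, unhides the scene, moves the active party to four slots and possesses itself.
; SpawnEnemies, not called here, makes a weighted random pick from EncounterTable and async-loads up to four enemy classes, spawning all at Enemy1's transform.
; GetBattleCharacters returns both parties as one list.
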(event `StartBattle`
  (params (ReturnPawn :type "Pawn Object Reference"))
  (set `self.ReturnPawn` ReturnPawn)
  (`self.SetActorHiddenInGame` false)
  (`self.MovePartyToBattle`)
  (`Controller.Possess` (`GameplayStatics.GetPlayerController` 0) self))

(event `MovePartyToBattle`
  (bind _aspc_tbrpg (cast `/Game/BattleSystem/TBRPG/PC_TBRPG` (`GameplayStatics.GetPlayerController` 0)))
  (bind _output_get (set `self.PlayerController` _aspc_tbrpg))
  (for (_array_element _array_index) (`/Game/BattleSystem/TBRPG/PC_TBRPG.ActiveParty` _output_get)
    (`self.K2_SetActorTransform` _array_element (`SceneComponent.K2_GetComponentToWorld` (`|GetArrayItem` (`|MakeArray` (`self.Player1`) (`self.Player2`) (`self.Player3`) (`self.Player4`)) _array_index)) false false)
    (`self.SetActorHiddenInGame` _array_element false)))

(event `SpawnEnemies`
  (bind _out_row (`self.PickEnemyLayout`))
  (`|ExecutionSequence`
    (:`then_0`
      (bind _class (`|LoadAssetClass` (`.EnemyClass1_5_B60B4C72444D48F6C7D473999044E3EE` (break `/Game/BattleSystem/TBRPG/Structs/S_EnemyEncounter` _out_row)))
        (:`Completed`
          (bind _asactor (castclass `Actor` _class))
          (bind _returnvalue (`|SpawnActorFromClass` _asactor (`SceneComponent.K2_GetComponentToWorld` (`self.Enemy1`)) "Undefined" "MultiplyWithRoot" null null))
          (`KismetArrayLibrary.Array_AddUnique` (`self.EnemyParty`) _returnvalue))))
    (:`then_1`
      (bind _class_2 (`|LoadAssetClass` (`.EnemyClass2_7_9445FD7441711045AA02AC9FA52D139C` (break `/Game/BattleSystem/TBRPG/Structs/S_EnemyEncounter` _out_row)))
        (:`Completed`
          (bind _asactor_2 (castclass `Actor` _class_2))
          (bind _returnvalue_2 (`|SpawnActorFromClass` _asactor_2 (`SceneComponent.K2_GetComponentToWorld` (`self.Enemy1`)) "Undefined" "MultiplyWithRoot" null null))
          (`KismetArrayLibrary.Array_AddUnique` (`self.EnemyParty`) _returnvalue_2))))
    (:`then_2`
      (bind _class_3 (`|LoadAssetClass` (`.EnemyClass3_9_9BA72CC64402D3EE259C359EDD45D421` (break `/Game/BattleSystem/TBRPG/Structs/S_EnemyEncounter` _out_row)))
        (:`Completed`
          (bind _asactor_3 (castclass `Actor` _class_3))
          (bind _returnvalue_3 (`|SpawnActorFromClass` _asactor_3 (`SceneComponent.K2_GetComponentToWorld` (`self.Enemy1`)) "Undefined" "MultiplyWithRoot" null null))
          (`KismetArrayLibrary.Array_AddUnique` (`self.EnemyParty`) _returnvalue_3))))
    (:`then_3`
      (bind _class_4 (`|LoadAssetClass` (`.EnemyClass4_11_75F55F3647EBF5D6CA92DD9D463EC4FE` (break `/Game/BattleSystem/TBRPG/Structs/S_EnemyEncounter` _out_row)))
        (:`Completed`
          (bind _asactor_4 (castclass `Actor` _class_4))
          (bind _returnvalue_4 (`|SpawnActorFromClass` _asactor_4 (`SceneComponent.K2_GetComponentToWorld` (`self.Enemy1`)) "Undefined" "MultiplyWithRoot" null null))
          (`KismetArrayLibrary.Array_AddUnique` (`self.EnemyParty`) _returnvalue_4))))))

(fn `GetBattleCharacters`
  (returns (BattleActors :type "Array of Actor Object Reference"))
  (locals (OutputArray :type "Array of Actor Object Reference"))
  (set `local.OutputArray` (`/Game/BattleSystem/TBRPG/PC_TBRPG.ActiveParty` (`self.PlayerController`)))
  (for _array_element (`self.EnemyParty`)
    (`KismetArrayLibrary.Array_AddUnique` (`local.OutputArray`) _array_element))
  (return (`local.OutputArray`)))

(fn `PickEnemyLayout`
  (returns (`Out Row` :type "/Game/BattleSystem/TBRPG/Structs/S_EnemyEncounter Structure"))
  (locals (TotalWeight :type "Float (double-precision)") (CountUpWeight :type "Float (double-precision)") (TargetWeight :type "Float (double-precision)"))
  (bind _encountertable (`self.EncounterTable`))
  (bind _encountertable_2 (`self.EncounterTable`))
  (if (== (`DataTableFunctionLibrary.GetDataTableRowStruct` _encountertable) "/Game/BattleSystem/TBRPG/Structs/S_EnemyEncounter.S_EnemyEncounter")
    (bind _outrownames (`DataTableFunctionLibrary.GetDataTableRowNames` _encountertable))
    (for _array_element _outrownames
      (bind _returnvalue (`|GetDataTableRow` _encountertable _array_element)
        (:`then`
          (set `local.TotalWeight` (+ (`local.TotalWeight`) (`.Weight_2_AF10BE1A49CF0F9A0AB854A39CDF616A` (break `/Game/BattleSystem/TBRPG/Structs/S_EnemyEncounter` _returnvalue)))))))
    (set `local.TargetWeight` (`KismetMathLibrary.RandomFloatInRange` 0.0 (`local.TotalWeight`)))
    (bind _outrownames_2 (`DataTableFunctionLibrary.GetDataTableRowNames` _encountertable_2))
    (for _array_element_2 _outrownames_2
      (bind _returnvalue_2 (`|GetDataTableRow` _encountertable_2 _array_element_2)
        (:`then`
          (bind _output_get (set `local.CountUpWeight` (+ (`local.CountUpWeight`) (`.Weight_2_AF10BE1A49CF0F9A0AB854A39CDF616A` (break `/Game/BattleSystem/TBRPG/Structs/S_EnemyEncounter` _returnvalue_2)))))
          (if (<= (`local.TargetWeight`) _output_get)
            (return _returnvalue_2)))))))

(fn `UserConstructionScript`)