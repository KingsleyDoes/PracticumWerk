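; Base pawn for turn-based RPG battle characters, with a flipbook sprite and an ability component.
; On BeginPlay it applies a random Haste offset to itself and grants the Wait ability.
; Turn and targeting events swap the sprite's outline overlay material, restoring the active-turn outline when untargeted during its turn.
; Helpers expose the ability component and reset the combat idle flipbook, while debug keys lower and print LP.
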(event EventBeginPlay
  (Default|AffectSelf (Variables|Default|GetAC_AbilityComponent) "NewEnumerator0" "Haste" "NewEnumerator4" "NewEnumerator0" (Math|Random|RandomFloatinRange -2.0 2.0))
  (Default|GiveAbility (Variables|Default|GetAC_AbilityComponent) "/Game/BattleSystem/TBRPG/Abilties/BP_TBAbility_Wait.BP_TBAbility_Wait_C"))

(event EventSetTurnActive
  (params (IsActive :type Boolean))
  (bind _sprite (Variables|Default|GetSprite))
  (if IsActive
    (Rendering|Material|SetOverlayMaterial _sprite "/Game/BattleSystem/TBRPG/Materials/M_Outliner.M_Outliner" :!class /Script/Engine.MeshComponent)
    (else
      (Rendering|Material|SetOverlayMaterial _sprite 0 :!class /Script/Engine.MeshComponent))))

(event EventSetTargeted
  (params (IsTargeted :type Boolean))
  (bind _sprite (Variables|Default|GetSprite))
  (if IsTargeted
    (Rendering|Material|SetOverlayMaterial _sprite "/Game/BattleSystem/TBRPG/Materials/M_OutlinerTarg.M_OutlinerTarg" :!class /Script/Engine.MeshComponent)
    (elif (Variables|/Game/BattleSystem/TBRPG/Abilties/AC_AbilityComponent.AC_AbilityComponent_C|GetIsTurn (Variables|Default|GetAC_AbilityComponent))
      (Rendering|Material|SetOverlayMaterial _sprite "/Game/BattleSystem/TBRPG/Materials/M_Outliner.M_Outliner" :!class /Script/Engine.MeshComponent)
      (else
        (Rendering|Material|SetOverlayMaterial _sprite 0 :!class /Script/Engine.MeshComponent)))))

(event Input|KeyboardEvents|DebugKeyF
  (params (Key :type Key%20Structure :default "None") (ActionValue :type Input%20Action%20Value%20Structure))
  (:Pressed
    (Default|AffectSelf (Variables|Default|GetAC_AbilityComponent) "NewEnumerator0" "LP" "NewEnumerator4" "NewEnumerator0" -1e+01)))

(event Input|KeyboardEvents|DebugKeyG
  (params (Key :type Key%20Structure :default "None") (ActionValue :type Input%20Action%20Value%20Structure))
  (:Pressed
    (bind _currentvaluewithmods (Default|GetAttributeCurrent (Variables|Default|GetAC_AbilityComponent) "None"))
    (Development|PrintText (Utilities|Text|FormatText "Player Has {LP} LP" _currentvaluewithmods))))

(fn ConstructionScript)

(fn ResetFlipbook
  (Sprite|SetFlipbook (Variables|Default|GetSprite) (Variables|Default|GetCombatIdle)))

(fn GetAbilityComponent
  (return (Variables|Default|GetAC_AbilityComponent)))