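; Parent Blueprint for player pawns in the TBRPG battle system, adding XP and level progression.
; GainXP accumulates TotalXP and reads XPCurve, calling LevelUP when the floored result exceeds the current Level.
; LevelUP stores the new level, then applies that level's LP, BP and Haste values from per-stat lookups through the ability component's AffectSelf.
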(fn `GainXP`
  (params (XPReceived :type Integer))
  (bind _output_get (set `self.TotalXP` (+ (`self.TotalXP`) XPReceived)))
  (bind _returnvalue (`KismetMathLibrary.FFloor` (`CurveFloat.GetFloatValue` (`self.XPCurve`) (`KismetMathLibrary.Conv_IntToDouble` _output_get))))
  (if (> _returnvalue (`self.Level`))
    (`self.LevelUP` _returnvalue)))

(fn `LevelUP`
  (params (NewLevel :type Integer))
  (bind _ac_abilitycomponent (`self.AC_AbilityComponent`))
  (bind _output_get (set `self.Level` NewLevel))
  (bind _returnvalue (- _output_get 0))
  (`/Game/BattleSystem/TBRPG/Abilties/AC_AbilityComponent.AffectSelf` _ac_abilitycomponent "NewEnumerator0" "LP" "NewEnumerator2" "NewEnumerator2" (`|GetArrayItem` (`self.LPCurve`) _returnvalue) 0)
  (`/Game/BattleSystem/TBRPG/Abilties/AC_AbilityComponent.AffectSelf` _ac_abilitycomponent "NewEnumerator0" "BP" "NewEnumerator2" "NewEnumerator2" (`|GetArrayItem` (`self.BPCurve`) _returnvalue) 0)
  (`/Game/BattleSystem/TBRPG/Abilties/AC_AbilityComponent.AffectSelf` _ac_abilitycomponent "NewEnumerator0" "Haste" "NewEnumerator2" "NewEnumerator2" (`|GetArrayItem` (`self.HasteCurve`) _returnvalue) 0))

(fn `UserConstructionScript`
  (`parent.UserConstructionScript`))