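; PC_TBRPG, likely the player controller for the turn-based RPG battle system, creates the player's party.
; On BeginPlay it spawns Galypso, Niren, Mehzia and Obi pawns at its own transform and keeps a reference to each.
; It hides all four in game, then stores them as the ActiveParty array.
; An unconnected spawn for a fifth member, Krania, uses the generic BP_PawnBase and never runs.
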(event `self.ReceiveBeginPlay`
  (bind _returnvalue (`self.GetTransform`))
  (bind _array (`|MakeArray` (`self.Galypso (P1)`) (`self.Niren (P2)`) (`self.Mehzia (P3)`) (`self.Obi (P4)`) :!type "Actor Object Reference"))
  (bind _returnvalue_2 (`|SpawnActorFromClass` "/Game/BattleSystem/TBRPG/CharactersBlueprints/BP_PawnBase_PlayerParent_Galypso.BP_PawnBase_PlayerParent_Galypso_C" _returnvalue "Undefined" "MultiplyWithRoot" null false "Galypso" null))
  (set `self.Galypso (P1)` _returnvalue_2)
  (bind _returnvalue_3 (`|SpawnActorFromClass` "/Game/BattleSystem/TBRPG/CharactersBlueprints/BP_PawnBase_PlayerParent_Niren.BP_PawnBase_PlayerParent_Niren_C" _returnvalue "Undefined" "MultiplyWithRoot" null false "Niren" null))
  (set `self.Niren (P2)` _returnvalue_3)
  (bind _returnvalue_4 (`|SpawnActorFromClass` "/Game/BattleSystem/TBRPG/CharactersBlueprints/BP_PawnBase_PlayerParent_Mehzia.BP_PawnBase_PlayerParent_Mehzia_C" _returnvalue "Undefined" "MultiplyWithRoot" null false "Mehza" null))
  (set `self.Mehzia (P3)` _returnvalue_4)
  (bind _returnvalue_5 (`|SpawnActorFromClass` "/Game/BattleSystem/TBRPG/CharactersBlueprints/BP_PawnBase_PlayerParent_Obi.BP_PawnBase_PlayerParent_Obi_C" _returnvalue "Undefined" "MultiplyWithRoot" null false "Obi" null))
  (set `self.Obi (P4)` _returnvalue_5)
  (for _array_element _array
    (`self.SetActorHiddenInGame` _array_element true))
  (set `self.ActiveParty` _array))

(fn `UserConstructionScript`)