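; Parent Blueprint for enemy pawns in the turn-based RPG battle system.
; When its ability component signals that a turn has started, it starts the StateTree logic, which drives the enemy's turn.
; A SetTargeted event shows or hides the ArrowSlot component to mark whether the enemy is currently targeted.
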(event `self.AC_AbilityComponent.TurnStarted`
  (`BrainComponent.StartLogic` (`self.StateTree`)))

(event `/Game/BattleSystem/TBRPG/BPI_TurnBasedCombat.SetTargeted`
  (params (IsTargeted :type Boolean))
  (bind _arrowslot (`self.ArrowSlot`))
  (if IsTargeted
    (`SceneComponent.SetHiddenInGame` _arrowslot false false)
    (else
      (`SceneComponent.SetHiddenInGame` _arrowslot true false))))

(fn `UserConstructionScript`
  (`parent.UserConstructionScript`))