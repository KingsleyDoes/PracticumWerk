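; BP_CampSky is an environment-art actor, apparently the camp sky backdrop, that animates vertically along with a linked tilemap.
; BeginPlay places it at a hardcoded raised position, and Settilemap stores the tilemap reference.
; Animate plays a Timeline that lerps both the sky and the tilemap from that raised position to a lower one, using identical absolute world locations.
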(event `Settilemap`
  (params (TM :type "PaperTileMapActor Object Reference"))
  (set `self.TM` TM))

(event `self.ReceiveBeginPlay`
  (`self.K2_SetActorLocation` self (80.0 -2000.0 2500.0) false false))

(event `Animate`
  (bind (_direction _newtrack_0) (`Timeline|Timeline` :!via `PlayFromStart`)
    (:`Update`
      (bind _returnvalue (`KismetMathLibrary.VLerp` (80.0 -2000.0 2500.0) (80.0 -2000.0 900.0) _newtrack_0))
      (`self.K2_SetActorLocation` self _returnvalue false false)
      (`self.K2_SetActorLocation` (`self.TM`) _returnvalue false false))))

(fn `UserConstructionScript`)