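; BP_EquipmentMesh is a static mesh equipment slot for the turn-based RPG battle system, showing the equipped item and applying its stat modifiers.
; Equip accepts only equipment matching its SlotName, clears the previous item, then sets the new mesh.
; Each modifier becomes a self-targeted effect through the owner's ability component, stored in Effects.
; Unequip ends those stored effects and clears both the item and mesh.
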(event `Equip`
  (params (Equipment :type "/Game/BattleSystem/TBRPG/Items/BP_EquipmentDataAsset Object Reference"))
  (if (== (`/Game/BattleSystem/TBRPG/Items/BP_EquipmentDataAsset.SlotName` Equipment) (`self.SlotName`))
    (`self.Unequip`)
    (set `self.CurrentlyEquipped` Equipment)
    (bind _component (message `/Game/BattleSystem/TBRPG/BPI_TurnBasedCombat.GetAbilityComponent` (`self.GetOwner`)))
    (for _array_element (`/Game/BattleSystem/TBRPG/Items/BP_EquipmentDataAsset.modifiers` (`self.CurrentlyEquipped`))
      (bind _effectreference (`/Game/BattleSystem/TBRPG/Abilties/AC_AbilityComponent.AffectSelf` _component "NewEnumerator3" (break `/Game/BattleSystem/TBRPG/Structs/S_AttributeModifier` _array_element) (`.StatValues_12_8AA6F93D47E8055C65BEA38AF8B6CB5F` (break `/Game/BattleSystem/TBRPG/Structs/S_AttributeModifier` _array_element)) (`.Opporation_14_0F6E555D4AD6FF1D4D615089D34F5A95` (break `/Game/BattleSystem/TBRPG/Structs/S_AttributeModifier` _array_element)) (`.Magnitude_13_50D1101C4D2D5554B305FD897B7BB871` (break `/Game/BattleSystem/TBRPG/Structs/S_AttributeModifier` _array_element)) 0))
      (`KismetArrayLibrary.Array_AddUnique` (`self.Effects`) _effectreference))
    (`self.SetStaticMesh` (`/Game/BattleSystem/TBRPG/Items/BP_EquipmentDataAsset.Mesh` (`self.CurrentlyEquipped`)))))

(event `Unequip`
  (bind _effects (`self.Effects`))
  (for _array_element _effects
    (`/Game/BattleSystem/TBRPG/BPO_TurnEffect.EndEffect` _array_element))
  (`KismetArrayLibrary.Array_Clear` _effects)
  (set `self.CurrentlyEquipped` null)
  (`self.SetStaticMesh` null))