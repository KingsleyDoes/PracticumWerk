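; BP_TBAbility is an ability actor for the turn-based RPG battle system, with an empty ActivateAbility event that acts as a hook for specific abilities.
; CommitAbility asks the owning ability component whether the cost is affordable, then deducts it from the cost's attribute through AffectSelf, or destroys the actor and returns false.
; EndAbility broadcasts an end dispatcher with itself, then destroys the actor.
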(event `ActivateAbility`)

(event `EndAbility`
  (`self.AbilityEndDisp` self)
  (`self.K2_DestroyActor`))

(fn `CommitAbility`
  (returns (Comitted :type Boolean))
  (bind (_cost_cost _cost_attributeused) (break `/Game/BattleSystem/TBRPG/Structs/S_AttributeCost` (`self.Cost`)))
  (bind _cando (`/Game/BattleSystem/TBRPG/BFL_RPGFunctions.CanDoAbility` (`self.OwningAbilityComponent`) (`self.Cost`)))
  (if _cando
    (`/Game/BattleSystem/TBRPG/AC_AbilityComponent.AffectSelf` (`self.OwningAbilityComponent`) "NewEnumerator0" _cost_attributeused "NewEnumerator4" "NewEnumerator0" (* _cost_cost -1.0) 0)
    (return true)
    (else
      (`self.K2_DestroyActor`)
      (return false))))

(fn `UserConstructionScript`)