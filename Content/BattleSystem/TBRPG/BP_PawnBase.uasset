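; Base pawn for the turn-based RPG battle system that carries an ability component and exposes it through GetAbilityComponent.
; On BeginPlay it grants the test ability BP_TBAbility_Test to that component.
; Debug key F applies a negative LP effect to the pawn itself.
; Debug key G prints a current attribute value labeled as LP, though the lookup passes None as the attribute name.
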(event EventBeginPlay
  (Default|GiveAbility (Variables|Default|GetAC_AbilityComponent) "/Game/BattleSystem/TBRPG/BP_TBAbility_Test.BP_TBAbility_Test_C"))

(event Collision|EventActorBeginOverlap
  (params (OtherActor :type Actor%20Object%20Reference)))

(event EventTick
  (params (DeltaSeconds :type Float%20%28single-precision%29)))

(event Input|KeyboardEvents|DebugKeyF
  (params (Key :type Key%20Structure :default "None") (ActionValue :type Input%20Action%20Value%20Structure))
  (:Pressed
    (Default|AffectSelf (Variables|Default|GetAC_AbilityComponent) "NewEnumerator0" "LP" "NewEnumerator4" "NewEnumerator0" -1e+01)))

(event Input|KeyboardEvents|DebugKeyG
  (params (Key :type Key%20Structure :default "None") (ActionValue :type Input%20Action%20Value%20Structure))
  (:Pressed
    (bind _currentvaluewithmods (Default|GetAttributeCurrent (Variables|Default|GetAC_AbilityComponent) "None"))
    (Development|PrintText (Utilities|Text|FormatText "Player Has {LP} LP" _currentvaluewithmods))))

(fn ConstructionScript)

(fn GetAbilityComponent
  (return (Variables|Default|GetAC_AbilityComponent)))