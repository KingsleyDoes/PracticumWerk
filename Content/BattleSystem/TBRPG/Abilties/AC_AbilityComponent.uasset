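; Ability component for turn-based RPG battles, managing an actor's attributes, abilities, effects and turn state.
; Owned abilities spawn as actors that enter selection or activate directly, with end events bound.
; Effects are BPO_TurnEffect objects: Instant and Temporary apply immediately, while Duration and Infinite join the applying component's active list, even for other targets, and run on StartTurn.
; Attribute getters add modifiers to base values, and dispatchers broadcast attribute and turn changes.
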(fn `ActivateOwnedAbility`
  (params (AbilityClass :type "/Game/BattleSystem/TBRPG/Abilties/BP_TBAbility Class Reference") (Event :type "Delegate (by ref)"))
  (returns (ReturnedAbility :type "/Game/BattleSystem/TBRPG/Abilties/BP_TBAbility Object Reference"))
  (if (`KismetArrayLibrary.Array_Contains` (`self.OwnedAbilities`) AbilityClass)
    (bind _spawnedability (`self.ActivateSingleAbility` AbilityClass Event))
    (return _spawnedability)
    (else
      (return null))))

(fn `ActivateSingleAbility`
  (params (AbilityClass :type "/Game/BattleSystem/TBRPG/Abilties/BP_TBAbility Class Reference") (Event :type "Delegate (by ref)") (SkipSelection :type Boolean))
  (returns (SpawnedAbility :type "/Game/BattleSystem/TBRPG/Abilties/BP_TBAbility Object Reference"))
  (bind _returnvalue (`self.GetOwner`))
  (bind _returnvalue_2 (`|SpawnActorFromClass` AbilityClass (`Actor.GetTransform` _returnvalue) "Undefined" "MultiplyWithRoot" _returnvalue self null))
  (`KismetArrayLibrary.Array_AddUnique` (`self.ActiveAbilities`) _returnvalue_2)
  (add `/Game/BattleSystem/TBRPG/Abilties/BP_TBAbility.AbilityEndDisp` _returnvalue_2 Event)
  (add `/Game/BattleSystem/TBRPG/Abilties/BP_TBAbility.AbilityEndDisp` _returnvalue_2 (`|CreateDelegate` :!event `EndTurn`))
  (if SkipSelection
    (`/Game/BattleSystem/TBRPG/Abilties/BP_TBAbility.ActivateAbility` _returnvalue_2)
    (else
      (`/Game/BattleSystem/TBRPG/Abilties/BP_TBAbility.SelectAbility` _returnvalue_2)))
  (return _returnvalue_2))

(fn `AffectSelf`
  (params (EffectType :type "/Game/BattleSystem/TBRPG/Enums/Enum_EffectType Enum" :default "NewEnumerator0") (AttributeAffected :type Name) (TargetStat :type "/Game/BattleSystem/TBRPG/Enums/Enum_TargetStats Enum" :default "NewEnumerator0") (AffectMath :type "/Game/BattleSystem/TBRPG/Enums/Enum_AffectMath Enum" :default "NewEnumerator0") (Magnitude :type "Float (double-precision)") (EffectTurnCounter :type Integer))
  (returns (EffectReference :type "/Game/BattleSystem/TBRPG/BPO_TurnEffect Object Reference"))
  (bind _effectreference (`self.ApplyEffectToTarget` EffectType self AttributeAffected TargetStat AffectMath Magnitude EffectTurnCounter))
  (return _effectreference))

(fn `ApplyEffectToTarget`
  (params (EffectType :type "/Game/BattleSystem/TBRPG/Enums/Enum_EffectType Enum" :default "NewEnumerator0") (TargetComponent :type "/Game/BattleSystem/TBRPG/Abilties/AC_AbilityComponent Object Reference") (AttributeAffected :type Name) (TargetStat :type "/Game/BattleSystem/TBRPG/Enums/Enum_TargetStats Enum" :default "NewEnumerator0") (AffectMath :type "/Game/BattleSystem/TBRPG/Enums/Enum_AffectMath Enum" :default "NewEnumerator0") (Magnitude :type "Float (double-precision)") (EffectTurnCounter :type Integer))
  (returns (EffectReference :type "/Game/BattleSystem/TBRPG/BPO_TurnEffect Object Reference"))
  (bind _returnvalue (`|GenericCreateObject` TargetComponent "/Game/BattleSystem/TBRPG/BPO_TurnEffect.BPO_TurnEffect_C" EffectType TargetComponent AttributeAffected TargetStat AffectMath Magnitude EffectTurnCounter))
  (add `/Game/BattleSystem/TBRPG/BPO_TurnEffect.UpdateAttributes` _returnvalue (`|CreateDelegate` TargetComponent :!event `OnAttributeUpdated`))
  (switch `/Game/BattleSystem/TBRPG/Enums/Enum_EffectType` (`local.EffectType`)
    (:`NewEnumerator0`
      (`/Game/BattleSystem/TBRPG/BPO_TurnEffect.ApplyEffect` _returnvalue :!label _label))
    (:`NewEnumerator1`
      (`KismetArrayLibrary.Array_AddUnique` (`self.ActiveEffects`) _returnvalue :!label _label_2))
    (:`NewEnumerator2`
      (goto _label_2))
    (:`NewEnumerator3`
      (goto _label)))
  (return _returnvalue))

(fn `EndTurn`
  (params (TurnAbility :type "/Game/BattleSystem/TBRPG/Abilties/BP_TBAbility Object Reference"))
  (`KismetArrayLibrary.Array_RemoveItem` (`self.ActiveAbilities`) TurnAbility)
  (set `self.IsTurn` false)
  (`self.TurnEnded`))

(fn `GetAttributeCurrent`
  (params (AttributeName :type Name))
  (returns (CurrentValueWithMods :type "Float (double-precision)"))
  (for _array_element (`self.Attributes`)
    (if (== AttributeName (break `/Game/BattleSystem/TBRPG/Structs/S_Attributes` _array_element))
      (bind (_minvalue _minvaluemod _maxvalue _maxvaluemod _currentvalue _currentvaluemod) (break `/Game/BattleSystem/TBRPG/Structs/S_Stats` (`.StatStruct_8_DC48FF6643B8809F86CE03B0B2EAB56A` (break `/Game/BattleSystem/TBRPG/Structs/S_Attributes` _array_element))))
      (return (+ _currentvalue _currentvaluemod)))))

(fn `GetAttributeMax`
  (params (AttributeName :type Name))
  (returns (MaxValueWithMods :type "Float (double-precision)"))
  (for _array_element (`self.Attributes`)
    (if (== AttributeName (break `/Game/BattleSystem/TBRPG/Structs/S_Attributes` _array_element))
      (bind (_minvalue _minvaluemod _maxvalue _maxvaluemod) (break `/Game/BattleSystem/TBRPG/Structs/S_Stats` (`.StatStruct_8_DC48FF6643B8809F86CE03B0B2EAB56A` (break `/Game/BattleSystem/TBRPG/Structs/S_Attributes` _array_element))))
      (return (+ _maxvalue _maxvaluemod)))))

(fn `GetAttributeMin`
  (params (AttributeName :type Name))
  (returns (MinValueWithMods :type "Float (double-precision)"))
  (for _array_element (`self.Attributes`)
    (if (== AttributeName (break `/Game/BattleSystem/TBRPG/Structs/S_Attributes` _array_element))
      (bind (_minvalue _minvaluemod) (break `/Game/BattleSystem/TBRPG/Structs/S_Stats` (`.StatStruct_8_DC48FF6643B8809F86CE03B0B2EAB56A` (break `/Game/BattleSystem/TBRPG/Structs/S_Attributes` _array_element))))
      (return (+ _minvalue _minvaluemod)))))

(fn `GiveAbility`
  (params (NewItem :type "/Game/BattleSystem/TBRPG/Abilties/BP_TBAbility Class Reference"))
  (`KismetArrayLibrary.Array_AddUnique` (`self.OwnedAbilities`) NewItem))

(fn `OnAttributeUpdated`
  (params (Attrib :type "/Game/BattleSystem/TBRPG/Structs/S_Attributes Structure"))
  (`self.AttributeDispatched` Attrib))

(fn `RemoveAbility`
  (params (Item :type "/Game/BattleSystem/TBRPG/Abilties/BP_TBAbility Class Reference"))
  (`KismetArrayLibrary.Array_RemoveItem` (`self.OwnedAbilities`) Item))

(fn `StartTurn`
  (for _array_element (`self.ActiveEffects`)
    (`/Game/BattleSystem/TBRPG/BPO_TurnEffect.ApplyEffect` _array_element))
  (set `self.IsTurn` true)
  (`self.TurnStarted`))