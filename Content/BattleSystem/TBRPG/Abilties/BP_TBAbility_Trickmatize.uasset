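; Turn-based RPG ability Trickmatize, which applies a negative LP effect to the owner's current target.
; On activation it commits the ability, then casts the owning ability component's target actor to BP_PawnBase.
; It fetches that pawn's ability component and applies a fixed LP reduction through the owner's component, then ends after a short delay.
; A failed commit or cast stops the graph before EndAbility is reached.
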(event `self.ActivateAbility`
  (bind _owningabilitycomponent (`self.OwningAbilityComponent`))
  (bind _comitted (`self.CommitAbility`))
  (if _comitted
    (bind _asbp_pawn_base (cast `/Game/BattleSystem/TBRPG/Characters/BP_PawnBase` (`/Game/BattleSystem/TBRPG/Abilties/AC_AbilityComponent.TargActor` _owningabilitycomponent)))
    (bind _component (message `/Game/BattleSystem/TBRPG/BPI_TurnBasedCombat.GetAbilityComponent` _asbp_pawn_base))
    (`/Game/BattleSystem/TBRPG/Abilties/AC_AbilityComponent.ApplyEffectToTarget` _owningabilitycomponent "NewEnumerator0" _component "LP" "NewEnumerator4" "NewEnumerator0" -5.0 0)
    (`KismetSystemLibrary.Delay` 2.0)
    (`self.EndAbility`)))

(fn `UserConstructionScript`
  (`parent.UserConstructionScript`))