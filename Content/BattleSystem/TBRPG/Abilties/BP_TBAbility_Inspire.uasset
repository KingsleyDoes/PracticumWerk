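; BP_TBAbility_Inspire is a turn-based RPG ability that applies a level-scaled BP effect to a targeted player pawn.
; On activation it commits, then casts the owning ability component's target to the player pawn class.
; It spawns a Niagara effect at the target and applies a magnitude derived from that target's Level.
; The ability ends after a short delay; a failed cast stops execution without calling EndAbility.
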(event `self.ActivateAbility`
  (bind _owningabilitycomponent (`self.OwningAbilityComponent`))
  (bind _targactor (`/Game/BattleSystem/TBRPG/Abilties/AC_AbilityComponent.TargActor` _owningabilitycomponent))
  (bind _comitted (`self.CommitAbility`))
  (if _comitted
    (bind _asbp_pawn_base (cast `/Game/BattleSystem/TBRPG/Characters/BP_PawnBase` _targactor))
    (bind _component (message `/Game/BattleSystem/TBRPG/BPI_TurnBasedCombat.GetAbilityComponent` _asbp_pawn_base))
    (bind _asbp_pawn_base_player_parent_obi (cast `/Game/BattleSystem/TBRPG/Characters/BP_PawnBase_PlayerParent_Obi` _asbp_pawn_base))
    (`NiagaraFunctionLibrary.SpawnSystemAtLocation` (`self.NiagaraSys`) (`self.K2_GetActorLocation` _targactor))
    (`/Game/BattleSystem/TBRPG/Abilties/AC_AbilityComponent.ApplyEffectToTarget` _owningabilitycomponent "NewEnumerator0" _component "BP" "NewEnumerator4" "NewEnumerator0" (`KismetMathLibrary.Conv_IntToDouble` (* (+ (`/Game/BattleSystem/TBRPG/Characters/BP_PawnBase_PlayerParent.Level` _asbp_pawn_base_player_parent_obi) 1) 5)) 0)
    (`KismetSystemLibrary.Delay` 2.0)
    (`self.EndAbility`)))

(fn `UserConstructionScript`
  (`parent.UserConstructionScript`))