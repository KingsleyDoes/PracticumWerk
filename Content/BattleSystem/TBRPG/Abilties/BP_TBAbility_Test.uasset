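; BP_TBAbility_Test is a gameplay ability, named as a test, that makes the owning BP_PawnBase jump.
; On activation it commits the ability, ending at once if that fails, then triggers the jump and binds to the pawn's movement-mode-changed delegate.
; The ability ends when that delegate fires with the pawn's movement mode back to Walking.
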(event `self.ActivateAbility`
  (bind _comitted (`self.CommitAbility`))
  (if _comitted
    (bind _asbp_pawn_base (cast `/Game/BattleSystem/TBRPG/CharactersBlueprints/BP_PawnBase` (`self.GetOwner`)))
    (`Character.Jump` _asbp_pawn_base)
    (add `Character.MovementModeChangedDelegate` _asbp_pawn_base (delegate `MovementModeChangedDelegate_Event`))
    (else
      (`self.EndAbility`))))

(event `MovementModeChangedDelegate_Event`
  (params (Character :type "Character Object Reference") (PrevMovementMode :type "EMovementMode Enum" :default "MOVE_None") (PreviousCustomMode :type Byte))
  (if (`|EnumEquality` (`CharacterMovementComponent.MovementMode` (`Character.CharacterMovement` (stale `self.ActivateAbility` _asbp_pawn_base))) "MOVE_Walking")
    (`self.EndAbility`)))

(fn `UserConstructionScript`
  (`parent.UserConstructionScript`))