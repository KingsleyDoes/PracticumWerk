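; Punch ability for the turn-based RPG battle system that damages the owning ability component's target actor.
; On activation it commits, plays a flipbook on the target pawn's effect animation, then applies a negative LP effect through the target's ability component.
; Damage scales with the target's own Level, and the target must be a Mehzia player pawn.
; After a two-second delay it clears the flipbook and ends.
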(event `self.ActivateAbility`
  (bind _owningabilitycomponent (`self.OwningAbilityComponent`))
  (bind _comitted (`self.CommitAbility`))
  (if _comitted
    (bind _asbp_pawn_base (cast `/Game/BattleSystem/TBRPG/CharactersBlueprints/BP_PawnBase` (`/Game/BattleSystem/TBRPG/Abilties/AC_AbilityComponent.TargActor` _owningabilitycomponent)))
    (bind _effectanimation (`/Game/BattleSystem/TBRPG/CharactersBlueprints/BP_PawnBase.EffectAnimation` _asbp_pawn_base))
    (`PaperFlipbookComponent.SetFlipbook` _effectanimation (`self.Flipbook`))
    (bind _component (message `/Game/BattleSystem/TBRPG/BPI_TurnBasedCombat.GetAbilityComponent` _asbp_pawn_base))
    (bind _asbp_pawn_base_player_parent_mehzia (cast `/Game/BattleSystem/TBRPG/CharactersBlueprints/BP_PawnBase_PlayerParent_Mehzia` _asbp_pawn_base))
    (`/Game/BattleSystem/TBRPG/Abilties/AC_AbilityComponent.ApplyEffectToTarget` _owningabilitycomponent "NewEnumerator0" _component "LP" "NewEnumerator4" "NewEnumerator0" (`KismetMathLibrary.Conv_IntToDouble` (* (+ (`/Game/BattleSystem/TBRPG/CharactersBlueprints/BP_PawnBase_PlayerParent.Level` _asbp_pawn_base_player_parent_mehzia) 1) -5)) 0)
    (`KismetSystemLibrary.Delay` 2.0)
    (`PaperFlipbookComponent.SetFlipbook` _effectanimation null)
    (`self.EndAbility`)))

(fn `UserConstructionScript`
  (`parent.UserConstructionScript`))