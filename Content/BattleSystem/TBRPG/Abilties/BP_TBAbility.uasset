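; Base ability actor for a turn-based RPG, with empty select and activate events and an end event that calls a dispatcher and destroys it.
; CommitAbility deducts the cost through the owning ability component, or destroys the actor if unaffordable.
; Targeting helpers move selection within or between player and enemy parties using a modulo wrap-around search.
; CanSelect filters that search and returns true by default, while UpdateSelectedTarg replaces unselectable targets.
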(event `SelectAbility`)

(event `ActivateAbility`)

(event `EndAbility`
  (`self.AbilityEndDisp` self)
  (`self.K2_DestroyActor`))

(fn `CanSelect`
  (params (CheckedActor :type "Actor Object Reference"))
  (returns (CanSelect :type Boolean))
  (return true))

(fn `CommitAbility`
  (returns (Comitted :type Boolean))
  (bind (_cost_cost _cost_attributeused) (break `/Game/BattleSystem/TBRPG/Structs/S_AttributeCost` (`self.Cost`)))
  (bind _cando (`/Game/BattleSystem/TBRPG/BFL_RPGFunctions.CanDoAbility` (`self.OwningAbilityComponent`) (`self.Cost`)))
  (if _cando
    (`/Game/BattleSystem/TBRPG/Abilties/AC_AbilityComponent.AffectSelf` (`self.OwningAbilityComponent`) "NewEnumerator0" _cost_attributeused "NewEnumerator4" "NewEnumerator0" (* _cost_cost -1.0) 0)
    (return true)
    (else
      (`self.K2_DestroyActor`)
      (return false))))

(fn `LoopOverArrayWithWrap`
  (params (LArray :type "Array of Actor Object Reference") (CountDown :type Boolean) (StartIndex :type Integer))
  (returns (OutputPin :type "Actor Object Reference"))
  (locals (StartingIndex :type Integer) (GoalIndex :type Integer) (CurrIndex :type Integer))
  (bind _returnvalue (`KismetArrayLibrary.Array_Length` LArray))
  (bind _countdown (`local.CountDown`))
  (bind _currindex (`local.CurrIndex`))
  (bind _currindex_2 (`local.CurrIndex`))
  (bind _goalindex (`local.GoalIndex`))
  (bind _output_get (set `local.StartingIndex` (+ StartIndex _returnvalue)))
  (set `local.GoalIndex` (+ _output_get (* (`KismetMathLibrary.SelectInt` -1 1 CountDown) _returnvalue)))
  (bind _output_get_2 (set `local.CurrIndex` (`local.StartingIndex`)))
  (bind _output (`|GetArrayItem` (`local.LArray`) (mod _output_get_2 _returnvalue)))
  (bind _canselect (`self.CanSelect` _output :!label _label))
  (if _canselect
    (return _output)
    (else
      (if _countdown
        (`/Engine/EditorBlueprintResources/StandardMacros.DecrementInt` _currindex
          (:`  `
            _))
        (else
          (`/Engine/EditorBlueprintResources/StandardMacros.IncrementInt` _currindex
            (:`  `
              _))))
      (if (select `bool` _countdown :`false` (> _currindex_2 _goalindex) :`true` (< _currindex_2 _goalindex))
        (return null)
        (else
          (goto _label))))))

(fn `SelectDown`
  (params (PlayerParty :type "Array of Actor Object Reference") (EnemyParty :type "Array of Actor Object Reference") (CurrSelected :type "Actor Object Reference"))
  (returns (OutputPin :type "Actor Object Reference"))
  (if (`KismetArrayLibrary.Array_Contains` PlayerParty (`local.CurrSelected`))
    (bind _outputpin (`self.LoopOverArrayWithWrap` PlayerParty false (+ (`KismetArrayLibrary.Array_Find` PlayerParty CurrSelected) 1)))
    (return _outputpin)
    (else
      (bind _outputpin_2 (`self.LoopOverArrayWithWrap` EnemyParty false (+ (`KismetArrayLibrary.Array_Find` EnemyParty CurrSelected) 1)))
      (return _outputpin_2))))

(fn `SelectOtherParty`
  (params (PlayerParty :type "Array of Actor Object Reference") (EnemyParty :type "Array of Actor Object Reference") (CurrSelected :type "Actor Object Reference"))
  (returns (OutputPin :type "Actor Object Reference"))
  (if (`KismetArrayLibrary.Array_Contains` PlayerParty (`local.CurrSelected`))
    (bind _outputpin (`self.LoopOverArrayWithWrap` EnemyParty false (`KismetArrayLibrary.Array_Find` PlayerParty CurrSelected)))
    (return _outputpin)
    (else
      (bind _outputpin_2 (`self.LoopOverArrayWithWrap` PlayerParty false (`KismetArrayLibrary.Array_Find` EnemyParty CurrSelected)))
      (return _outputpin_2))))

(fn `SelectUp`
  (params (PlayerParty :type "Array of Actor Object Reference") (EnemyParty :type "Array of Actor Object Reference") (CurrSelected :type "Actor Object Reference"))
  (returns (OutputPin :type "Actor Object Reference"))
  (if (`KismetArrayLibrary.Array_Contains` (`local.PlayerParty`) (`local.CurrSelected`))
    (bind _outputpin (`self.LoopOverArrayWithWrap` PlayerParty true (- (`KismetArrayLibrary.Array_Find` PlayerParty CurrSelected) 1)))
    (return _outputpin)
    (else
      (bind _outputpin_2 (`self.LoopOverArrayWithWrap` EnemyParty true (- (`KismetArrayLibrary.Array_Find` EnemyParty CurrSelected) 1)))
      (return _outputpin_2))))

(fn `UpdateSelectedTarg`
  (params (PlayerParty :type "Array of Actor Object Reference") (EnemyParty :type "Array of Actor Object Reference") (CurrSelected :type "Actor Object Reference"))
  (returns (OutputPin :type "Actor Object Reference"))
  (bind _returnvalue (`KismetArrayLibrary.Array_Find` PlayerParty CurrSelected))
  (bind _returnvalue_2 (`KismetArrayLibrary.Array_Find` EnemyParty CurrSelected))
  (bind _canselect (`self.CanSelect` CurrSelected))
  (if _canselect
    (return CurrSelected)
    (elif (`KismetArrayLibrary.Array_Contains` PlayerParty CurrSelected)
      (bind _outputpin (`self.LoopOverArrayWithWrap` PlayerParty false _returnvalue))
      (`/Engine/EditorBlueprintResources/StandardMacros.IsValid` _outputpin
        (:`Is Valid`
          (return _outputpin))
        (:`Is Not Valid`
          (bind _outputpin_2 (`self.LoopOverArrayWithWrap` (`local.EnemyParty`) false _returnvalue))
          (return _outputpin_2)))
      (else
        (bind _outputpin_3 (`self.LoopOverArrayWithWrap` EnemyParty false _returnvalue_2))
        (`/Engine/EditorBlueprintResources/StandardMacros.IsValid` _outputpin_3
          (:`Is Valid`
            (return _outputpin_3))
          (:`Is Not Valid`
            (bind _outputpin_4 (`self.LoopOverArrayWithWrap` (`local.PlayerParty`) false _returnvalue_2))
            (return _outputpin_4)))))))

(fn `UserConstructionScript`)