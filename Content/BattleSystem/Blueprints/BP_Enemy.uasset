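; Enemy actor for the battle system that opens the fight UI when the top-down player character touches its hitbox.
; On overlap it reaches the HUD through player controller 0, shows FIGHTUI and calls BattleBEGIN.
; Ending the overlap only hides the fight UI.
; A custom EnemyDeath event destroys the actor; nothing in this Blueprint calls it.
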(event `self.Hitbox.OnComponentBeginOverlap`
  (params (OverlappedComponent :type "PrimitiveComponent Object Reference") (OtherActor :type "Actor Object Reference") (OtherComp :type "PrimitiveComponent Object Reference") (OtherBodyIndex :type Integer) (bFromSweep :type Boolean) (SweepResult :type "HitResult Structure (by ref)"))
  (cast `/Game/TopDown/Blueprints/BP_TopDownCharacter` OtherActor)
  (bind _asbp_top_down_controller (cast `/Game/TopDown/Blueprints/BP_TopDownController` (`GameplayStatics.GetPlayerController` 0)))
  (bind _hud (`/Game/TopDown/Blueprints/BP_TopDownController.HUD` _asbp_top_down_controller))
  (`Widget.SetVisibility` (`/Game/BattleSystem/Blueprints/W_HUD.FIGHT_UI` _hud) "Visible")
  (`/Game/BattleSystem/Blueprints/W_HUD.BattleBEGIN` _hud))

(event `self.Hitbox.OnComponentEndOverlap`
  (params (OverlappedComponent :type "PrimitiveComponent Object Reference") (OtherActor :type "Actor Object Reference") (OtherComp :type "PrimitiveComponent Object Reference") (OtherBodyIndex :type Integer))
  (cast `/Game/TopDown/Blueprints/BP_TopDownCharacter` OtherActor)
  (bind _asbp_top_down_controller (cast `/Game/TopDown/Blueprints/BP_TopDownController` (`GameplayStatics.GetPlayerController` 0)))
  (`Widget.SetVisibility` (`/Game/BattleSystem/Blueprints/W_HUD.FIGHT_UI` (`/Game/TopDown/Blueprints/BP_TopDownController.HUD` _asbp_top_down_controller)) "Hidden"))

(event `EnemyDeath`
  (`self.K2_DestroyActor`))

(fn `UserConstructionScript`)