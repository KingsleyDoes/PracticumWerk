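; Battle game mode that sets up the fight and runs a queue-based turn system for party and enemy units.
; On BeginPlay it switches to the battle camera, caches both unit lists and, after a short delay, adds party units to the player controller's HUD.
; Turn requests join a duplicate-free queue, with a DoOnce gate admitting one turn at a time through each unit's combat component until ReadyNextTurn resets it.
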(event `self.ReceiveBeginPlay`
  (bind _returnvalue (`GameplayStatics.GetActorOfClass` "/Game/BattleSystem/Blueprints/BP_Camera_Battle.BP_Camera_Battle_C"))
  (bind _output_get (set `self.Main Battle Cam` _returnvalue))
  (`PlayerController.SetViewTargetWithBlend` (`GameplayStatics.GetPlayerController` 0) _output_get 0.0 "VTBlend_Linear" 0.0 false)
  (bind _outactors (`GameplayStatics.GetAllActorsOfClass` "/Game/BattleSystem/Blueprints/Units/C_PartyUnit.C_PartyUnit_C"))
  (set `self.PartyUnits` _outactors)
  (bind _outactors_2 (`GameplayStatics.GetAllActorsOfClass` "/Game/BattleSystem/Blueprints/Units/C_EnemyUnit.C_EnemyUnit_C"))
  (set `self.EnemyUnits` _outactors_2)
  ; added HUD to viewport
  (`KismetSystemLibrary.Delay` 0.2)
  (bind _asgm_battle_player_controller (cast `/Game/BattleSystem/Blueprints/GM_BattlePlayerController` (`GameplayStatics.GetPlayerController` 0)))
  (set `self.Battle HUD` (`/Game/BattleSystem/Blueprints/GM_BattlePlayerController.BattleHUD` _asgm_battle_player_controller))
  ; added units to HUD
  (for _array_element (`self.PartyUnits`)
    (`/Game/BattleSystem/Blueprints/W_HUD.AddPartyUnitToHUD` (`self.Battle HUD`) _array_element)))

(event `TurnRequest`
  (params (Unit :type "/Game/BattleSystem/Blueprints/Units/C_UnitBase Object Reference"))
  (`KismetArrayLibrary.Array_AddUnique` (`self.TurnOrder`) Unit)
  (`self.StartTurn`))

(event `StartTurn`
  (bind _bpc_combatcomponent (`/Game/BattleSystem/Blueprints/Units/C_UnitBase.BPC_CombatComponent` (`|GetArrayItem` (`self.TurnOrder`))))
  (`/Engine/EditorBlueprintResources/StandardMacros.DoOnce` false :!label _label
    (:`Completed`
      (if (`KismetArrayLibrary.Array_IsValidIndex` (`self.TurnOrder`))
        (`/Game/BattleSystem/Blueprints/BPC_CombatComponent.StartUnitTurn` _bpc_combatcomponent)
        (add `/Game/BattleSystem/Blueprints/BPC_CombatComponent.TurnEnded` _bpc_combatcomponent (`|CreateDelegate` :!event `ReadyNextTurn`))
        (`KismetArrayLibrary.Array_Remove` (`self.TurnOrder`))
        (else
          (`self.ReadyNextTurn`))))))

(event `ReadyNextTurn`
  (`|ExecutionSequence`
    (:`then_0`
      (goto _label :!via `Reset`))
    (:`then_1`
      (if (`KismetArrayLibrary.Array_IsValidIndex` (`self.TurnOrder`))
        (`self.StartTurn`)))))

(fn `UserConstructionScript`)