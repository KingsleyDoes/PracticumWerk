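; Combat component for battle units that schedules each unit's turn on a speed-based action timer.
; On BeginPlay it caches the owning C_UnitBase and its transform, then starts a timer whose delay shrinks from max to min action time as SPD rises.
; The timer requests a turn from GM_Battle.
; StartUnitTurn opens the battle menu for party units only; EndUnitTurn is an empty stub.
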(event `self.ReceiveBeginPlay`
  (bind _asc_unit_base (cast `/Game/BattleSystem/Blueprints/Units/C_UnitBase` (`self.GetOwner`)))
  (bind _output_get (set `self.UnitCharacter` _asc_unit_base))
  (set `self.BattlePosition` (`Actor.GetTransform` _output_get))
  (`self.BeginBattle`))

(fn `BeginBattle`
  (bind _returnvalue (`KismetSystemLibrary.K2_SetTimer` self "RequestTurn" (+ (* (- 1.0 (`KismetMathLibrary.NormalizeToRange` (`self.SPD`) 1.0 50.0)) (- (`self.MaxActionTime`) (`self.MinActionTime`))) (`self.MinActionTime`))))
  (set `self.ActionTimer` _returnvalue))

(fn `EndUnitTurn`)

(fn `RequestTurn`
  (bind _asgm_battle (cast `/Game/BattleSystem/Blueprints/GM_Battle` (`GameplayStatics.GetGameMode`)))
  (`/Game/BattleSystem/Blueprints/GM_Battle.TurnRequest` _asgm_battle (`self.UnitCharacter`)))

(fn `StartUnitTurn`
  (bind _unitcharacter (`self.UnitCharacter`))
  (if (`KismetMathLibrary.ClassIsChildOf` (`GameplayStatics.GetObjectClass` _unitcharacter) "/Game/BattleSystem/Blueprints/Units/C_PartyUnit.C_PartyUnit_C")
    (bind _returnvalue (`|CreateWidget` "/Game/Widgets/W_UnitBattleMenu.W_UnitBattleMenu_C" null _unitcharacter))
    (bind _output_get (set `self.ActionMenu` _returnvalue))
    (`UserWidget.AddToViewport` _output_get 0)))