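; GM_TurnBased is a game mode for a turn-based battle system that tracks whether it is the player's or the enemy's turn.
; BeginPlay creates the W_BattHUD widget for the first player controller and adds it to the viewport.
; SwitchTurn toggles CurrentTurn between the two sides, and the TestTurn event prints the active side as a debug check.
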(event `self.ReceiveBeginPlay`
  (bind _returnvalue (`|CreateWidget` "/Game/BattleSystem/NuSystem/W_BattHUD.W_BattHUD_C" (`GameplayStatics.GetPlayerController` 0)))
  (bind _output_get (set `self.HUD` _returnvalue))
  (`UserWidget.AddToViewport` _output_get 0))

(event `TestTurn`
  (switch `/Game/BattleSystem/NuSystem/Enum_TurnState` (`self.CurrentTurn`)
    (:`NewEnumerator0`
      (`KismetSystemLibrary.PrintText` "Player Turn"))
    (:`NewEnumerator1`
      (`KismetSystemLibrary.PrintText` "Enemy Turn"))))

(fn `SwitchTurn`
  (if (`|EnumEquality` "NewEnumerator0" (`self.CurrentTurn`))
    (set `self.CurrentTurn` "NewEnumerator1")
    (else
      (set `self.CurrentTurn` "NewEnumerator0"))))

(fn `UserConstructionScript`)