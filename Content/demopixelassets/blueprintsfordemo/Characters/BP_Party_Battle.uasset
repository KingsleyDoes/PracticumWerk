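; BP_Party_Battle represents the player's party in battle, showing Niren, Mehzia, Obi and Galypso as Paper2D flipbook sprites.
; BeginPlay adds the W_BattleHUD_v2 widget and calls StartRound, a placeholder for speed-based turn order.
; Tick reapplies every idle flipbook, while the main sprite's OnFinishedPlaying calls PlayIdle to loop and restart all but Obi.
; Mehzia's combat action events are empty stubs.
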(event `StartRound`
  (`KismetSystemLibrary.PrintString` "insert code here for determining order based on speed scores"))

(event `MehziaBasicAttack`
  ; Mehzia's Combat Actions
)

(event `MehziaRally`
  ; Mehzia's Combat Actions
)

(event `MehziaSneakAttack`
  ; Mehzia's Combat Actions
)

(event `self.ReceiveBeginPlay`
  (bind _returnvalue (`|CreateWidget` "/Game/demopixelassets/W_BattleHUD_v2.W_BattleHUD_v2_C"))
  (bind _output_get (set `self.BattleHUD` _returnvalue))
  (`UserWidget.AddToPlayerScreen` _output_get 0)
  (`self.StartRound`))

(event `self.Sprite.OnFinishedPlaying`
  (`PaperFlipbookComponent.SetFlipbook` (`self.Sprite`) "/Game/demopixelassets/customassets/niren/niren-testsprite-idle1.niren-testsprite-idle1")
  (`self.PlayIdle`))

(event `self.ReceiveTick`
  (params (DeltaSeconds :type "Float (single-precision)"))
  (`self.Updateanim`))

(fn `PlayIdle`
  (bind _galypso (`self.galypso`))
  (bind _sprite (`self.Sprite`))
  (bind _mehzia (`self.Mehzia`))
  (`PaperFlipbookComponent.SetLooping` _sprite true)
  (`PaperFlipbookComponent.SetLooping` _mehzia true)
  (`PaperFlipbookComponent.SetLooping` _galypso true)
  (if (not (`PaperFlipbookComponent.IsPlaying` _sprite))
    (`PaperFlipbookComponent.Play` _sprite)
    (`PaperFlipbookComponent.Play` _mehzia)
    (`PaperFlipbookComponent.Play` _galypso)))

(fn `Updateanim`
  (`PaperFlipbookComponent.SetFlipbook` (`self.Sprite`) "/Game/demopixelassets/customassets/niren/niren-testsprite-idle1.niren-testsprite-idle1")
  (`PaperFlipbookComponent.SetFlipbook` (`self.Mehzia`) "/Game/demopixelassets/customassets/Mehzia/mehzia-sprite-idle.mehzia-sprite-idle")
  (`PaperFlipbookComponent.SetFlipbook` (`self.Obi`) "/Game/demopixelassets/customassets/obi/obi-sprite-idle.obi-sprite-idle")
  (`PaperFlipbookComponent.SetFlipbook` (`self.galypso`) "/Game/demopixelassets/customassets/galypso/galypso-sprite-idle.galypso-sprite-idle"))

(fn `UserConstructionScript`)