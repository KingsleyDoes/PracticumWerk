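; BP_Party2d is a 2D party character that travels through a side-scrolling level with four flipbook-animated members.
; Space starts a timeline that lerps the capsule along X between fixed points, with bound stop and resume events pausing and continuing it.
; Tick picks run or idle flipbooks from the running flag, or jump and fall for the lead sprite when airborne.
; BeginPlay adds the travel HUD and gives background layers dynamic materials with per-layer parallax multipliers.
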(event `Key|SpaceBar`
  (params (Key :type "Key Structure"))
  (bind _capsulecomponent (`self.CapsuleComponent`))
  (bind (_returnvalue_x _returnvalue_y _returnvalue_z) (`KismetMathLibrary.BreakVector` (`SceneComponent.K2_GetComponentLocation` _capsulecomponent)))
  (:`Pressed`
    (add `self.stopMoving` (delegate `HaltMovement`))
    (add `self.ResumeMoving` (delegate `ResumeMovement`))
    (set `self.isrunning` true :!label _label)
    (bind (_direction _progress) (`Timeline|runthroughlevel` :!label _label_2)
      (:`Update`
        (bind _output_get (set `self.Progress` _progress))
        (`SceneComponent.K2_SetWorldLocation` _capsulecomponent (`KismetMathLibrary.VLerp` (`KismetMathLibrary.MakeVector` 1900.0 _returnvalue_y _returnvalue_z) (`KismetMathLibrary.MakeVector` 14500.0 _returnvalue_y _returnvalue_z) _output_get) false false))
      (:`Finished`
        (set `self.isrunning` false)))))

(event `ResumeMovement`
  (goto _label))

(event `HaltMovement`
  (set `self.isrunning` false)
  (goto _label_2 :!via `Stop`))

(event `self.ReceiveBeginPlay`
  (bind _returnvalue (`|CreateWidget` "/Game/Widgets/Travel_HUD.Travel_HUD_C"))
  (bind _output_get (set `self.TravelHUD` _returnvalue))
  (`UserWidget.AddToPlayerScreen` _output_get 0)
  (cast `PlayerController` (`self.GetController`))
  ;[0.08434 0.1062 0.15 0.5] Gets background layers and groups them into an array
  (for (_array_element _array_index) (`SceneComponent.GetChildrenComponents` (`self.staticbackground`) false)
    (bind _aspaper_sprite_component (cast `PaperSpriteComponent` _array_element))
    (bind _returnvalue_2 (`PrimitiveComponent.CreateDynamicMaterialInstance` _aspaper_sprite_component 0 null "None"))
    (`KismetArrayLibrary.Array_Add` (`self.DynamicLayers`) _returnvalue_2)
    (`MaterialInstanceDynamic.SetScalarParameterValue` _returnvalue_2 "ParallaxMult" (`|GetArrayItem` (`self.ParallaxMultipliers`) _array_index))))

(event `self.Sprite.OnFinishedPlaying`
  (`PaperFlipbookComponent.SetFlipbook` (`self.Sprite`) "/Game/BattleSystem/TBRPG/PixelAssets/CharacterArt/niren/niren-testsprite-idle1.niren-testsprite-idle1")
  (`self.PlayIdle`))

(event `self.ReceiveTick`
  (params (DeltaSeconds :type "Float (single-precision)"))
  (`self.Updateanim`))

(fn `PlayIdle`
  (bind _galypso (`self.galypso`))
  (bind _sprite (`self.Sprite`))
  (bind _mehzia (`self.Mehzia`))
  (`PaperFlipbookComponent.SetLooping` _sprite true)
  (`PaperFlipbookComponent.SetLooping` _mehzia true)
  (`PaperFlipbookComponent.SetLooping` _galypso true)
  (if (not (`PaperFlipbookComponent.IsPlaying` _sprite))
    (`PaperFlipbookComponent.Play` _sprite)
    (`PaperFlipbookComponent.Play` _mehzia)
    (`PaperFlipbookComponent.Play` _galypso)))

(fn `Updateanim`
  (bind (_returnvalue_x _returnvalue_y _returnvalue_z) (`KismetMathLibrary.BreakVector` (`self.GetVelocity`)))
  (bind _sprite (`self.Sprite`))
  (bind _sprite_2 (`self.Sprite`))
  (bind _mehzia (`self.Mehzia`))
  (bind _galypso (`self.galypso`))
  (bind _obi (`self.Obi`))
  (if (`NavMovementComponent.IsMovingOnGround` (`self.CharacterMovement`))
    (if (`self.isrunning`)
      (`PaperFlipbookComponent.SetFlipbook` _sprite_2 "/Game/BattleSystem/TBRPG/PixelAssets/CharacterArt/niren/niren-testsprite-run1.niren-testsprite-run1")
      (`PaperFlipbookComponent.SetFlipbook` _mehzia "/Game/BattleSystem/TBRPG/PixelAssets/CharacterArt/Mehzia/mehzia-sprite-run.mehzia-sprite-run")
      (`PaperFlipbookComponent.SetFlipbook` _obi "/Game/BattleSystem/TBRPG/PixelAssets/CharacterArt/obi/obi-sprite-run.obi-sprite-run")
      (`PaperFlipbookComponent.SetFlipbook` _galypso "/Game/BattleSystem/TBRPG/PixelAssets/CharacterArt/galypso/galypso-sprite-run.galypso-sprite-run")
      (else
        (`PaperFlipbookComponent.SetFlipbook` _sprite_2 "/Game/BattleSystem/TBRPG/PixelAssets/CharacterArt/niren/niren-testsprite-idle1.niren-testsprite-idle1")
        (`PaperFlipbookComponent.SetFlipbook` _mehzia "/Game/BattleSystem/TBRPG/PixelAssets/CharacterArt/Mehzia/mehzia-sprite-idle.mehzia-sprite-idle")
        (`PaperFlipbookComponent.SetFlipbook` _obi "/Game/BattleSystem/TBRPG/PixelAssets/CharacterArt/obi/obi-sprite-idle.obi-sprite-idle")
        (`PaperFlipbookComponent.SetFlipbook` _galypso "/Game/BattleSystem/TBRPG/PixelAssets/CharacterArt/galypso/galypso-sprite-idle.galypso-sprite-idle")))
    (elif (< _returnvalue_z -100.0)
      (`PaperFlipbookComponent.SetFlipbook` _sprite "/Game/demopixelassets/flipbooks/FB_Fall.FB_Fall")
      (else
        (`PaperFlipbookComponent.SetFlipbook` _sprite "/Game/demopixelassets/flipbooks/FB_Jump.FB_Jump")))))

(fn `UserConstructionScript`)