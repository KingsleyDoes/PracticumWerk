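; Paper2D follower character that reacts to the demo player character entering or leaving its PlayerDetector.
; It flips around on BeginPlay and on detector entry; on exit it copies the player's rotation, with delayed updates to the NearPlayer flag.
; A MoveForward event supplies forward movement input.
; Each tick, Updateanim picks the flipbook from ground state and velocity, though both grounded branches have no flipbook assigned.
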(event `self.ReceiveBeginPlay`
  (`self.turn`))

(event `MoveForward`
  (`self.AddMovementInput` (`self.GetActorForwardVector`)))

(event `self.ReceiveTick`
  (params (DeltaSeconds :type "Float (single-precision)"))
  (`self.Updateanim`))

(event `self.PlayerDetector.OnComponentBeginOverlap`
  (params (OverlappedComponent :type "PrimitiveComponent Object Reference") (OtherActor :type "Actor Object Reference") (OtherComp :type "PrimitiveComponent Object Reference") (OtherBodyIndex :type Integer) (bFromSweep :type Boolean) (SweepResult :type "HitResult Structure (by ref)"))
  (cast `/Game/demopixelassets/blueprintsfordemo/Characters/BP_Papercharacter_DemoCharacter` OtherActor)
  (`self.turn`)
  (`KismetSystemLibrary.Delay` 0.2)
  (set `self.NearPlayer` true))

(event `self.PlayerDetector.OnComponentEndOverlap`
  (params (OverlappedComponent :type "PrimitiveComponent Object Reference") (OtherActor :type "Actor Object Reference") (OtherComp :type "PrimitiveComponent Object Reference") (OtherBodyIndex :type Integer))
  (bind _asbp_papercharacter_demo_character (cast `/Game/demopixelassets/blueprintsfordemo/Characters/BP_Papercharacter_DemoCharacter` OtherActor))
  (`KismetSystemLibrary.Delay` 0.2)
  (`self.K2_SetActorRotation` self (`self.K2_GetActorRotation` _asbp_papercharacter_demo_character) false)
  (set `self.NearPlayer` false))

(fn `turn`
  (`self.K2_SetActorRotation` (`KismetMathLibrary.ComposeRotators` (`self.K2_GetActorRotation`) (struct :`Yaw` 180.0))))

(fn `Updateanim`
  (bind (_returnvalue_x _returnvalue_y _returnvalue_z) (`KismetMathLibrary.BreakVector` (`self.GetVelocity`)))
  (bind _sprite (`self.Sprite`))
  (bind _sprite_2 (`self.Sprite`))
  (if (`NavMovementComponent.IsMovingOnGround` (`self.CharacterMovement`))
    (if (> (`KismetMathLibrary.VSize` (`self.GetVelocity`)) 0.0)
      (`PaperFlipbookComponent.SetFlipbook` _sprite_2 null)
      (else
        (`PaperFlipbookComponent.SetFlipbook` _sprite_2 null)))
    (elif (< _returnvalue_z -100.0)
      (`PaperFlipbookComponent.SetFlipbook` _sprite "/Game/demopixelassets/flipbooks/FB_Fall.FB_Fall")
      (else
        (`PaperFlipbookComponent.SetFlipbook` _sprite "/Game/demopixelassets/flipbooks/FB_Jump.FB_Jump")))))

(fn `UserConstructionScript`)