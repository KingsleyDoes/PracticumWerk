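; Playable side-scrolling Paper2D character Galypso for free-roam, with Enhanced Input movement along X, yaw flipping to face travel direction, and jumping.
; Each tick picks an idle, run or float flipbook from ground state and velocity.
; An overlap component stores uncompleted BPI_Interact actors for the interact input, while Enter advances a stored NPC's widget.
; Parallax background layer setup is present but unconnected.
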(event `self.ReceiveBeginPlay`
  (bind _asplayer_controller (cast `PlayerController` (`self.GetController`)))
  (`EnhancedInputSubsystemInterface.AddMappingContext` (pcsubsystem `EnhancedInputLocalPlayerSubsystem` _asplayer_controller) "/Game/demopixelassets/blueprintsfordemo/inputs/IA_Inputdemo.IA_Inputdemo" 0 (struct)))

(event `self.Sprite.OnFinishedPlaying`
  (`PaperFlipbookComponent.SetFlipbook` (`self.Sprite`) "/Game/demopixelassets/customassets/galypso/galypso-sprite-idle.galypso-sprite-idle")
  (`self.PlayIdle`))

(event `self.ReceiveTick`
  (params (DeltaSeconds :type "Float (single-precision)"))
  (`self.Updateanim`))

(event `EnhancedInput|/Game/demopixelassets/blueprintsfordemo/inputs/IA_Jumpdemo`
  (params (ActionValue :type Boolean) (ElapsedSeconds :type "Float (double-precision)") (TriggeredSeconds :type "Float (double-precision)") (InputAction :type "InputAction Object Reference" :default "/Game/demopixelassets/blueprintsfordemo/inputs/IA_Jumpdemo.IA_Jumpdemo"))
  (:`Started`
    (`self.Jump`))
  (:`Completed`
    (`self.StopJumping`)))

(event `EnhancedInput|/Game/demopixelassets/blueprintsfordemo/inputs/IA_Move`
  (params (ActionValue :type "Float (double-precision)") (ElapsedSeconds :type "Float (double-precision)") (TriggeredSeconds :type "Float (double-precision)") (InputAction :type "InputAction Object Reference" :default "/Game/demopixelassets/blueprintsfordemo/inputs/IA_Move.IA_Move"))
  (:`Triggered`
    (`self.AddMovementInput` (1.0 0.0 0.0) ActionValue)
    (`Controller.SetControlRotation` (`self.GetController`) (select `bool` (> ActionValue 0.0) :`false` (`KismetMathLibrary.MakeRotator` 0.0 0.0 180.0) :`true` (`KismetMathLibrary.MakeRotator` 0.0)))))

(event `self.InteractOverlap.OnComponentBeginOverlap`
  (params (OverlappedComponent :type "PrimitiveComponent Object Reference") (OtherActor :type "Actor Object Reference") (OtherComp :type "PrimitiveComponent Object Reference") (OtherBodyIndex :type Integer) (bFromSweep :type Boolean) (SweepResult :type "HitResult Structure (by ref)"))
  (if (`KismetSystemLibrary.DoesImplementInterface` OtherActor "/Game/demopixelassets/blueprintsfordemo/InterfacesAndComponenets/BPI_Interact.BPI_Interact_C")
    (bind _completed (message `/Game/demopixelassets/blueprintsfordemo/InterfacesAndComponenets/BPI_Interact.GetCompleted` OtherActor))
    (if (not _completed)
      (set `self.OverlappingActor` true)
      (set `self.InteractableParty` OtherActor))))

(event `self.InteractOverlap.OnComponentEndOverlap`
  (params (OverlappedComponent :type "PrimitiveComponent Object Reference") (OtherActor :type "Actor Object Reference") (OtherComp :type "PrimitiveComponent Object Reference") (OtherBodyIndex :type Integer))
  (if (`KismetSystemLibrary.DoesImplementInterface` OtherActor "/Game/demopixelassets/blueprintsfordemo/InterfacesAndComponenets/BPI_Interact.BPI_Interact_C")
    (set `self.OverlappingActor` false)
    (set `self.InteractableParty` null)))

(event `EnhancedInput|/Game/demopixelassets/blueprintsfordemo/inputs/IA_Interact`
  (params (ActionValue :type Boolean) (ElapsedSeconds :type "Float (double-precision)") (TriggeredSeconds :type "Float (double-precision)") (InputAction :type "InputAction Object Reference" :default "/Game/demopixelassets/blueprintsfordemo/inputs/IA_Interact.IA_Interact"))
  (:`Triggered`
    (if (`self.OverlappingActor`)
      (message `/Game/demopixelassets/blueprintsfordemo/InterfacesAndComponenets/BPI_Interact.Interact` (`self.InteractableParty`) self))))

(event `EnhancedInput|/Game/demopixelassets/blueprintsfordemo/inputs/IA_Enter`
  (params (ActionValue :type Boolean) (ElapsedSeconds :type "Float (double-precision)") (TriggeredSeconds :type "Float (double-precision)") (InputAction :type "InputAction Object Reference" :default "/Game/demopixelassets/blueprintsfordemo/inputs/IA_Enter.IA_Enter"))
  (:`Completed`
    (bind _asbp_npcchild (cast `/Game/demopixelassets/blueprintsfordemo/Characters/BP_NPCchild` (`self.InteractableParty`)))
    (`/Engine/EditorBlueprintResources/StandardMacros.IsValid` _asbp_npcchild
      (:`Is Valid`
        (`/Game/Widgets/W_NPCspeech.PressedEnter` (`/Game/demopixelassets/blueprintsfordemo/Characters/BP_NPCparent.NPCwidget` _asbp_npcchild))))))

(fn `PlayIdle`
  (bind _sprite (`self.Sprite`))
  (`PaperFlipbookComponent.SetLooping` _sprite true)
  (if (not (`PaperFlipbookComponent.IsPlaying` _sprite))
    (`PaperFlipbookComponent.Play` _sprite)))

(fn `Updateanim`
  (bind (_returnvalue_x _returnvalue_y _returnvalue_z) (`KismetMathLibrary.BreakVector` (`self.GetVelocity`)))
  (bind _sprite (`self.Sprite`))
  (bind _sprite_2 (`self.Sprite`))
  (if (`NavMovementComponent.IsMovingOnGround` (`self.CharacterMovement`))
    (if (> (`KismetMathLibrary.VSize` (`self.GetVelocity`)) 0.0)
      (`PaperFlipbookComponent.SetFlipbook` _sprite_2 "/Game/demopixelassets/customassets/galypso/galypso-sprite-run.galypso-sprite-run")
      (else
        (`PaperFlipbookComponent.SetFlipbook` _sprite_2 "/Game/demopixelassets/customassets/galypso/galypso-sprite-idle.galypso-sprite-idle")))
    (elif (< _returnvalue_z -100.0)
      (`PaperFlipbookComponent.SetFlipbook` _sprite "/Game/demopixelassets/customassets/galypso/galypso-sprite-floatidle.galypso-sprite-floatidle")
      (else
        (`PaperFlipbookComponent.SetFlipbook` _sprite "/Game/demopixelassets/customassets/galypso/galypso-sprite-float.galypso-sprite-float")))))

(fn `UserConstructionScript`)