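; Paper2D player character for a side-scrolling pixel-art demo, with movement, jumping and flipbook animation.
; BeginPlay adds an Enhanced Input mapping context; move input pushes along world X and snaps controller yaw to face the travel direction, while jump input drives the standard Character jump.
; Each Tick, Updateanim selects the run, idle, jump or fall flipbook from ground state, speed and vertical velocity.
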(event `self.ReceiveBeginPlay`
  (bind _asplayer_controller (cast `PlayerController` (`self.GetController`)))
  (`EnhancedInputSubsystemInterface.AddMappingContext` (pcsubsystem `EnhancedInputLocalPlayerSubsystem` _asplayer_controller) "/Game/demopixelassets/blueprintsfordemo/inputs/IA_Inputdemo.IA_Inputdemo" 0 (struct)))

(event `EnhancedInput|/Game/demopixelassets/blueprintsfordemo/inputs/IA_Jumpdemo`
  (params (ActionValue :type Boolean) (ElapsedSeconds :type "Float (double-precision)") (TriggeredSeconds :type "Float (double-precision)") (InputAction :type "InputAction Object Reference" :default "/Game/demopixelassets/blueprintsfordemo/inputs/IA_Jumpdemo.IA_Jumpdemo"))
  (:`Started`
    (`self.Jump`))
  (:`Completed`
    (`self.StopJumping`)))

(event `self.ReceiveTick`
  (params (DeltaSeconds :type "Float (single-precision)"))
  (`self.Updateanim`))

(event `EnhancedInput|/Game/demopixelassets/blueprintsfordemo/inputs/IA_Move`
  (params (ActionValue :type "Float (double-precision)") (ElapsedSeconds :type "Float (double-precision)") (TriggeredSeconds :type "Float (double-precision)") (InputAction :type "InputAction Object Reference" :default "/Game/demopixelassets/blueprintsfordemo/inputs/IA_Move.IA_Move"))
  (:`Triggered`
    (`self.AddMovementInput` (1.0 0.0 0.0) ActionValue)
    (`Controller.SetControlRotation` (`self.GetController`) (select `bool` (> ActionValue 0.0) :`false` (`KismetMathLibrary.MakeRotator` 0.0 0.0 180.0) :`true` (`KismetMathLibrary.MakeRotator` 0.0)))))

(fn `Updateanim`
  (bind (_returnvalue_x _returnvalue_y _returnvalue_z) (`KismetMathLibrary.BreakVector` (`self.GetVelocity`)))
  (bind _sprite (`self.Sprite`))
  (bind _sprite_2 (`self.Sprite`))
  (if (`NavMovementComponent.IsMovingOnGround` (`self.CharacterMovement`))
    (if (> (`KismetMathLibrary.VSize` (`self.GetVelocity`)) 0.0)
      (`PaperFlipbookComponent.SetFlipbook` _sprite_2 "/Game/demopixelassets/flipbooks/FB_Player_Run.FB_Player_Run")
      (else
        (`PaperFlipbookComponent.SetFlipbook` _sprite_2 "/Game/demopixelassets/flipbooks/FB_Player_Idle.FB_Player_Idle")))
    (elif (< _returnvalue_z -100.0)
      (`PaperFlipbookComponent.SetFlipbook` _sprite "/Game/demopixelassets/flipbooks/FB_Fall.FB_Fall")
      (else
        (`PaperFlipbookComponent.SetFlipbook` _sprite "/Game/demopixelassets/flipbooks/FB_Jump.FB_Jump")))))

(fn `UserConstructionScript`)